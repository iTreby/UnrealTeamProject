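; BP_Enemy_Parent is a base enemy Blueprint that handles being hit by projectiles, losing health and dying.
; It caches its AI controller on BeginPlay; hits from BP_Projectile call ApplyDamage and latch an IsShot flag.
; AnyDamage subtracts from CurrentHealth and, at zero or below, runs death once: it plays the death animation, unpossesses the controller, disables capsule collision and sets a lifespan for delayed removal.
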(event EventBeginPlay
  (bind _asaicontroller (Utilities|Casting|CastToAIController (Pawn|GetController)))
  (Variables|Default|SetAIC _asaicontroller))

(event EventTick
  (params (DeltaSeconds :type Float%20%28single-precision%29)))

(event Collision|EventHit
  (params (MyComp :type Primitive%20Component%20Object%20Reference) (Other :type Actor%20Object%20Reference) (OtherComp :type Primitive%20Component%20Object%20Reference) (bSelfMoved :type Boolean) (HitLocation :type Vector :default "0, 0, 0") (HitNormal :type Vector :default "0, 0, 0") (NormalImpulse :type Vector :default "0, 0, 0") (Hit :type Hit%20Result%20Structure%20%28by%20ref%29))
  (Utilities|Casting|CastToBP_Projectile Other)
  (Game|Damage|ApplyDamage 0 0.0 0 0)
  (if (not (Variables|Default|GetisShot))
    (Variables|Default|SetisShot true)))

(event Game|Damage|EventAnyDamage
  (params (Damage :type Float%20%28single-precision%29) (DamageType :type Damage%20Type%20Object%20Reference) (InstigatedBy :type Controller%20Object%20Reference) (DamageCauser :type Actor%20Object%20Reference))
  ;[1 1 1] Take Dmg / Death
  (Variables|Default|SetcurrentHealth (- (Variables|Default|GetcurrentHealth) Damage))
  (if (<= (Variables|Default|GetcurrentHealth) 0.0)
    (if (not (Variables|Default|GetisDead))
      (Variables|Default|SetisDead true)
      (Components|Animation|PlayAnimation (Variables|Character|GetMesh) (Variables|Default|GetDeathAnim) false)
      (Pawn|UnPossess (Variables|Default|GetAIC))
      (Collision|SetCollisionEnabled (Variables|Collision|GetCapsuleComponent) "NoCollision")
      (Actor|SetLifeSpan 6e+01))))

(fn ConstructionScript)