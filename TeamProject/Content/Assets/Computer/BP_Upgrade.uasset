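; BP_Upgrade is an interactable shop actor, filed under Computer assets, that opens the player's shop menu.
; On interact it adds the ShopMenuWBP held by BP_Character to the viewport, shows the cursor, disables character movement and switches to UI-only input.
; Each tick it turns its TextRender toward the camera using the cached character's spring arm rotation with yaw flipped 180 degrees.
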(event Custom|CustomEvent)

(event EventOnInteract
  (bind _returnvalue (Game|GetPlayerController 0))
  (Development|PrintString "SHOP")
  (UserInterface|Viewport|AddtoViewport (Variables|/Game/CharacterBP/BP_Character.BP_Character_C|GetShopMenuWBP (stale EventBeginPlay _asbp_character)) 0)
  (Variables|/Script/Engine.PlayerController|SetbShowMouseCursor _returnvalue true)
  (Pawn|Components|CharacterMovement|DisableMovement (Variables|/Script/Engine.Character|GetCharacterMovement (stale EventBeginPlay _asbp_character)))
  (Input|SetInputModeUIOnly _returnvalue (Variables|/Game/CharacterBP/BP_Character.BP_Character_C|GetShopMenuWBP (stale EventBeginPlay _asbp_character)) "DoNotLock"))

(event EventBeginPlay
  (bind _asbp_character (Utilities|Casting|CastToBP_Character (Game|GetPlayerCharacter 0))))

(event EventTick
  (params (DeltaSeconds :type Float%20%28single-precision%29))
  (Transformation|SetWorldRotation (Variables|Default|GetTextRender) (Math|Rotator|MakeRotator (.roll (Transformation|GetWorldRotation (Variables|/Game/CharacterBP/BP_Character.BP_Character_C|GetSpringArm (stale EventBeginPlay _asbp_character)))) (.pitch (Transformation|GetWorldRotation (Variables|/Game/CharacterBP/BP_Character.BP_Character_C|GetSpringArm (stale EventBeginPlay _asbp_character)))) (+ (.yaw (Transformation|GetWorldRotation (Variables|/Game/CharacterBP/BP_Character.BP_Character_C|GetSpringArm (stale EventBeginPlay _asbp_character)))) 1.8e+02)) false false))

(fn ConstructionScript)