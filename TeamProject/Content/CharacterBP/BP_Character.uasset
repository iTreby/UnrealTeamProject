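; Player character for a shooter, handling movement, sprinting, aiming, weapon switching and HUD widgets.
; Number inputs swap rifle, pistol and orb gun by destroying and respawning a BP_Weapon_Parent actor on the hand socket, setting stance flags and ammo type.
; Firing requires aiming, which shows the crosshair, tightens pitch limits, slows walking and animates FOV via timeline.
; A blood overlay's opacity follows lost health, with a debug toggle on Q.
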(event Custom|SetBloodAlpha
  ;[1 1 1] Fire Weapon
  ;;[1 1 1] Temporary, find way to dynamically set (material?), so it is compatible with healing
  (Widget|SetRenderOpacity (Variables|Default|GetBloodWBP) (Math|Float|Clamp(Float) (- 1.0 (/ (Variables|Default|GetcurrentHP) (Variables|Default|GetmaxHP))))))

(event EventBeginPlay
  ;[1 1 1] Initialize
  (Utilities|FlowControl|Sequence
    (:then_0
      (CallFunction|ModifyMovement))
    (:then_1
      (bind _returnvalue (UserInterface|CreateWidget "/Game/CharacterBP/HUD/WBP_Crosshair.WBP_Crosshair_C"))
      (Variables|Default|SetCrosshair _returnvalue)
      (bind _returnvalue_2 (UserInterface|CreateWidget "/Game/CharacterBP/HUD/WBP_TakeDmg.WBP_TakeDmg_C"))
      (bind _output_get (Variables|Default|SetBloodWBP _returnvalue_2))
      (Widget|SetRenderOpacity _output_get 0.0)
      (UserInterface|Viewport|AddtoViewport _output_get 0)
      (bind _returnvalue_3 (UserInterface|CreateWidget "/Game/CharacterBP/HUD/WBP_Player.WBP_Player_C"))
      (UserInterface|Viewport|AddtoViewport _returnvalue_3 0)
      (bind _returnvalue_4 (UserInterface|CreateWidget "/Game/CharacterBP/HUD/WBP_EnergyBar.WBP_EnergyBar_C"))
      (Variables|Default|SetEnergyWBP _returnvalue_4))
    (:then_2
      (Variables|Default|SetinRifleStance true)
      (Variables|Default|SetcanSwitchWeapon true))
    (:then_3
      (CallFunction|AttachWeapon "/Game/CharacterBP/Weapons/BP_Rifle.BP_Rifle_C"))
    (:then_4
      (CallFunction|ClampCamera 5e+01 -4e+01))))

(event Collision|EventActorBeginOverlap
  (params (OtherActor :type Actor%20Object%20Reference)))

(event Input|ActionEvents|InputActionReloadWeapon
  (params (Key :type Key%20Structure :default "None"))
  ;[1 1 1] Fire Weapon
  (:Pressed
    (Default|ReloadWeapon (Variables|Default|GetCurrentWeapon))))

(event Input|ActionEvents|InputActionAim
  (params (Key :type Key%20Structure :default "None"))
  ;[1 1 1] Aiming / Field of View
  (:Pressed
    (if (Variables|Default|GetisSprinting)
      (Variables|Default|SetisSprinting false))
    (Variables|Default|SetisAiming true)
    (CallFunction|ModifyMovement)
    (CallFunction|ClampCamera 3e+01 -6e+01)
    (Variables|Default|SetcanShoot true)
    (UserInterface|Viewport|AddtoViewport (Variables|Default|GetCrosshair) 0)
    (bind _fieldofview (Timeline|Timeline_0 Play)
      (:Update
        (Camera|SetFieldOfView (Variables|Default|GetCamera) _fieldofview))))
  (:Released
    (Variables|Default|SetisAiming false)
    (CallFunction|ModifyMovement)
    (CallFunction|ClampCamera 5e+01 -4e+01)
    (Variables|Default|SetcanShoot false)
    (Widget|RemovefromParent (Variables|Default|GetCrosshair))
    (Timeline|Timeline_0 Reverse)))

(event Input|ActionEvents|InputActionSprint
  (params (Key :type Key%20Structure :default "None"))
  ;[1 1 1] Sprint
  (:Pressed
    (Variables|Default|SetcanSwitchWeapon false)
    (if (Variables|Default|GetisAiming)
      (Widget|RemovefromParent (Variables|Default|GetCrosshair)))
    (Variables|Default|SetisSprinting true)
    (CallFunction|ModifyMovement))
  (:Released
    (Variables|Default|SetcanSwitchWeapon true)
    (if (Variables|Default|GetisAiming)
      (if (UserInterface|Viewport|IsinViewport (Variables|Default|GetCrosshair))
        _
        (else
          (UserInterface|Viewport|AddtoViewport (Variables|Default|GetCrosshair) 0))))
    (Variables|Default|SetisSprinting false)
    (CallFunction|ModifyMovement)))

(event Input|ActionEvents|InputActionEquipWeapon3
  (params (Key :type Key%20Structure :default "None"))
  ;[1 1 1] Switch Weapons
  (:Pressed
    (if (Variables|Default|GetcanSwitchWeapon)
      (if (Variables|Default|GetinRifleStance)
        _
        (else
          (Variables|Default|SetinRifleStance true)
          (Variables|Default|SetInPistolStance false)))
      (CallFunction|ReplaceWeapon "/Game/CharacterBP/Weapons/BP_OrbGun.BP_OrbGun_C" (Variables|Default|GetorbClip)))))

(event Input|ActionEvents|InputActionEquipWeapon2
  (params (Key :type Key%20Structure :default "None"))
  ;[1 1 1] Switch Weapons
  (:Pressed
    (if (Variables|Default|GetcanSwitchWeapon)
      (if (Variables|Default|GetinRifleStance)
        (Variables|Default|SetinRifleStance false)
        (Variables|Default|SetInPistolStance true))
      (CallFunction|ReplaceWeapon "/Game/CharacterBP/Weapons/BP_Pistol.BP_Pistol_C" (Variables|Default|GetpistolClip)))))

(event Input|ActionEvents|InputActionEquipWeapon1
  (params (Key :type Key%20Structure :default "None"))
  ;[1 1 1] Switch Weapons
  (:Pressed
    (if true
      (if (Variables|Default|GetcanSwitchWeapon)
        (if (Variables|Default|GetinRifleStance)
          _
          (else
            (Variables|Default|SetinRifleStance true)
            (Variables|Default|SetInPistolStance false)))
        (CallFunction|ReplaceWeapon "/Game/CharacterBP/Weapons/BP_Rifle.BP_Rifle_C" (Variables|Default|GetrifleClip))))))

(event Input|ActionEvents|InputActionFireWeapon
  (params (Key :type Key%20Structure :default "None"))
  (bind _currentweapon (Variables|Default|GetCurrentWeapon))
  ;[1 1 1] Fire Weapon
  (:Pressed
    (if (and (Variables|Default|GetcanShoot) (Variables|Default|GetcanSwitchWeapon))
      (Default|FireWeapon _currentweapon)))
  (:Released
    (Default|StopFiring _currentweapon)))

(event Input|ActionEvents|InputActionEquipWeapon4
  (params (Key :type Key%20Structure :default "None"))
  ;[1 1 1] Switch Weapons
)

(event Input|AxisEvents|InputAxisMoveForward
  (params (AxisValue :type Float%20%28single-precision%29))
  ;[1 1 1] Character Controller
  (Pawn|Input|AddMovementInput (Math|Vector|GetForwardVector (Pawn|GetControlRotation :!class /Script/Engine.Pawn)) AxisValue false))

(event Input|AxisEvents|InputAxisMoveRight
  (params (AxisValue :type Float%20%28single-precision%29))
  ;[1 1 1] Character Controller
  (Pawn|Input|AddMovementInput (Math|Vector|GetRightVector (Pawn|GetControlRotation :!class /Script/Engine.Pawn)) AxisValue false))

(event Input|AxisEvents|InputAxisTurn
  (params (AxisValue :type Float%20%28single-precision%29))
  ;[1 1 1] Character Controller
  (Pawn|Input|AddControllerYawInput AxisValue))

(event Input|AxisEvents|InputAxisLookUp
  (params (AxisValue :type Float%20%28single-precision%29))
  ;[1 1 1] Character Controller
  (Pawn|Input|AddControllerPitchInput AxisValue))

(event Input|KeyboardEvents|Q
  (params (Key :type Key%20Structure :default "None"))
  (bind _bloodwbp (Variables|Default|GetBloodWBP))
  ;[1 1 1] Fire Weapon
  ;;[1 1 1] Temporary, find way to dynamically set (material?), so it is compatible with healing
  ;;;[1 1 1] Debug blood splat
  (:Pressed
    (Utilities|FlowControl|FlipFlop
      (:A
        (Widget|RemovefromParent _bloodwbp)
        (Development|PrintString "Hiding bloodscreen"))
      (:B
        (UserInterface|Viewport|AddtoViewport _bloodwbp 0)
        (Development|PrintString "Showing bloodscreen")))))

(fn ConstructionScript)

(fn ModifyMovement
  (bind _charactermovement (Variables|Character|GetCharacterMovement))
  (if (Variables|Default|GetisSprinting)
    ;[1 1 1] Run Speed
    (Variables|/Script/Engine.CharacterMovementComponent|SetMaxWalkSpeed _charactermovement 6e+02)
    (elif (Variables|Default|GetisAiming)
      ;[1 1 1] Aim Speed
      (Variables|/Script/Engine.CharacterMovementComponent|SetMaxWalkSpeed _charactermovement 175.0)
      (else
        ;[1 1 1] Walk Speed
        (Variables|/Script/Engine.CharacterMovementComponent|SetMaxWalkSpeed _charactermovement 2.5e+02)))))

(fn AttachWeapon
  (params (Weapon :type Actor%20Class%20Reference))
  ;[1 1 1] Attach Weapon
  (bind _returnvalue (Game|SpawnActorfromClass (Variables|Default|GetDesiredWeapon) (Transformation|GetActorTransform) "AlwaysSpawn" 0 0))
  (bind _asbp_weapon_parent (Utilities|Casting|CastToBP_Weapon_Parent _returnvalue))
  (bind _output_get (Variables|Default|SetCurrentWeapon _asbp_weapon_parent))
  (Transformation|AttachComponentToComponent _output_get (Variables|Character|GetMesh) "WeaponSocket" "SnapToTarget" "SnapToTarget" "KeepWorld" true)
  (Default|SetCamera _asbp_weapon_parent (Variables|Default|GetCamera)))

(fn ClampCamera
  (params (PitchMax :type Float%20%28single-precision%29) (PitchMin :type Float%20%28single-precision%29))
  (bind _returnvalue (Game|GetPlayerCameraManager 0))
  (Variables|/Script/Engine.PlayerCameraManager|SetViewPitchMax _returnvalue PitchMax)
  (Variables|/Script/Engine.PlayerCameraManager|SetViewPitchMin _returnvalue PitchMin))

(fn ReplaceWeapon
  (params (Weapon :type Actor%20Class%20Reference) (AmmoType :type Integer))
  (bind _energywbp (Variables|Default|GetEnergyWBP))
  ;[1 1 1] Attach Weapon
  (Actor|DestroyActor (Variables|Default|GetCurrentWeapon))
  (bind _returnvalue (Game|SpawnActorfromClass Weapon (Transformation|GetActorTransform) "AlwaysSpawn" 0 0))
  (bind _asbp_weapon_parent (Utilities|Casting|CastToBP_Weapon_Parent _returnvalue))
  (bind _output_get (Variables|Default|SetCurrentWeapon _asbp_weapon_parent))
  (Variables|/Game/CharacterBP/Weapons/BP_Weapon_Parent.BP_Weapon_Parent_C|SetCurrentAmmo _output_get AmmoType)
  (Transformation|AttachComponentToComponent _output_get (Variables|Character|GetMesh) "WeaponSocket" "SnapToTarget" "SnapToTarget" "KeepWorld" true)
  (Default|SetCamera _asbp_weapon_parent (Variables|Default|GetCamera))
  (if (UserInterface|Viewport|IsinViewport _energywbp)
    (Widget|RemovefromParent _energywbp)))