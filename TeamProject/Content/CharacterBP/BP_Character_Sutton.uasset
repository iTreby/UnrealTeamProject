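; Sutton player character: third-person movement, sprint and aim, weapon switching via spawned socket-attached actors, plus HUD, pause and game-over screens.
; Damage drains shield before HP, driving blood overlay, directional indicator and timer-based shield recharge.
; Abilities include a timed block field, shield-consuming energy slam and prototype teleport.
; Slow time costs HP, offsetting global dilation with player custom dilation and a faster rifle firing rate.
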(event OnComponentBeginOverlap(EnergyBombBox)
  (params (OverlappedComponent :type Primitive%20Component%20Object%20Reference) (OtherActor :type Actor%20Object%20Reference) (OtherComp :type Primitive%20Component%20Object%20Reference) (OtherBodyIndex :type Integer) (bFromSweep :type Boolean) (SweepResult :type Hit%20Result%20Structure%20%28by%20ref%29))
  (bind _energybombdmg (Variables|Default|GetenergyBombDmg))
  (bind _energybombdmg_2 (Variables|Default|GetenergyBombDmg))
  (bind _returnvalue (+ _energybombdmg 5e+01))
  (bind _returnvalue_2 (Math|Random|RandomFloatinRange _energybombdmg_2 _returnvalue))
  ;[0 1 0.04499] Attack
  ;;[0 1 0.3215] EnergySlam
  (Game|Damage|ApplyDamage OtherActor _returnvalue_2 0 self)
  (Camera|PlayWorldCameraShake "/Game/CharacterBP/HUD/BP_SlamShake.BP_SlamShake_C" (Transformation|GetActorLocation) 0.0 5e+02)
  (Components|Activation|Activate (Variables|Default|GetP_EnergyBomb) false)
  (Development|PrintString (Utilities|String|ToString(Float) _returnvalue_2)))

(event Custom|SetBloodAlpha
  ;[0 1 0.04499] Attack
  ;;[1 1 1] Blood splat
  (Widget|SetRenderOpacity (Variables|Default|GetBloodWBP) (Math|Float|Clamp(Float) (- 1.0 (/ (Variables|Default|GetcurrentHP) (Variables|Default|GetmaxHP))))))

(event Custom|TakeDamage
  (params (Damage :type Float%20%28single-precision%29) (WorldLoc :type Vector) (EnemyActorRef :type Actor%20Object%20Reference))
  (bind _dindicatorwbp (Variables|Default|GetDIndicatorWBP))
  (bind _dindicatorwbp_2 (Variables|Default|GetDIndicatorWBP))
  ;[0.07573 0.3843 1] TakeDamage
  ;;[1 1 1] TakeDamage(hp)
  ;;[1 1 1] TakeDamage(shield)
  (if (Variables|Default|GetIsBlockFieldActived)
    (Development|PrintString "Shield")
    (elif (> (Variables|Default|GetcurrentShield) 0.0)
      (if (> (- (Variables|Default|GetcurrentShield) Damage) 0.0)
        (Variables|Default|SetcurrentShield (- (Variables|Default|GetcurrentShield) Damage))
        (else
          (Variables|Default|SetcurrentShield 0.0)
          ;;;[1 1 1] Substract Shield Overkill Dmg from HP
          (Development|PrintString (Utilities|String|ToString(Float) (- Damage (Variables|Default|GetcurrentShield))) true true "(R=1.000000,G=0.180073,B=0.000000,A=1.000000)" 5.0)
          (Variables|Default|SetcurrentHP (- (Variables|Default|GetcurrentHP) (- Damage (Variables|Default|GetcurrentShield))))
          (CallFunction|SetBloodAlpha)))
      (CallFunction|Restoreshield :!label _label)
      ;;[0.2423 0.116 1] DmgIndicator
      ;;;[1 1 1] Damage Indicator
      (Class|Widget|SetRenderTransformAngle _dindicatorwbp (.Yaw (Math|Rotator|BreakRotator (Math|Rotator|Delta(Rotator) (Math|Rotator|FindLookatRotation (Transformation|GetActorLocation) WorldLoc) (Transformation|GetActorRotation)))))
      (if (UserInterface|Viewport|IsinViewport _dindicatorwbp)
        ;;;[1 1 1] Ensure widget lasts the same time per target
        (CallFunction|RestartIndicTimer)
        (else
          (UserInterface|Animation|PlayAnimation _dindicatorwbp_2 (Variables|/Game/CharacterBP/HUD/Images/WBP_DamageIndicator.WBP_DamageIndicator_C|GetfadeIn _dindicatorwbp_2) 0.0 1 "Forward" 1.0)
          (UserInterface|Viewport|AddtoViewport _dindicatorwbp_2 0)
          (bind _returnvalue (Utilities|Time|SetTimerbyEvent (delegate Custom|AdjustIndicator) 0.01 true))
          (CallFunction|RestartIndicTimer)))
      (elif (<= (Variables|Default|GetcurrentHP) 0.0)
        (Development|PrintString "Dead")
        (Utilities|FlowControl|Delay 1.0)
        (CallFunction|GameOver)
        (else
          (Variables|Default|SetcurrentHP (- (Variables|Default|GetcurrentHP) Damage))
          (CallFunction|SetBloodAlpha)
          (goto _label))))))

(event Custom|Restoreshield
  ;[0.07573 0.3843 1] TakeDamage
  ;;[1 1 1] TakeDamage(hp)
  ;;;[1 1 1] Restore Shield Logic
  (if (Variables|Default|GetshieldActivated)
    (Utilities|Time|ClearandInvalidateTimerbyHandle (Variables|Default|GetEnergyTimer))
    (Utilities|FlowControl|RetriggerableDelay (Variables|Default|GetshieldRegenDelay))
    (if (> (Variables|Default|GetcurrentHP) 0.0)
      (bind _returnvalue (Utilities|Time|SetTimerbyEvent (delegate Custom|TickShield) 0.025 true))
      (Variables|Default|SetEnergyTimer _returnvalue))))

(event Custom|TickShield
  ;[0.07573 0.3843 1] TakeDamage
  ;;[1 1 1] TakeDamage(hp)
  ;;;[1 1 1] Restore Shield Logic
  (if (!= (Variables|Default|GetcurrentShield) (Variables|Default|GetmaxShield))
    (Variables|Default|SetcurrentShield (+ (Variables|Default|GetcurrentShield) 1.25))
    (else
      (Utilities|Time|ClearandInvalidateTimerbyHandle (Variables|Default|GetEnergyTimer))
      (Development|PrintString "Shield Full -Recharge complete"))))

(event Custom|SlowEffect
  (bind _mesh (Variables|Character|GetMesh))
  (bind _returnvalue (Transformation|GetWorldTransform _mesh))
  ;[1 1 1] Slowtime Effect
  (Niagara|SpawnSystemAttached "/Game/CharacterBP/Character_Effect/Speed_NS.Speed_NS" _mesh "None" (.location _returnvalue) (.rotation _returnvalue) "KeepRelativeOffset" false))

(event Custom|AdjustIndicator
  ;[0.07573 0.3843 1] TakeDamage
  ;;[0.2423 0.116 1] DmgIndicator
  ;;;[1 1 1] Damage Indicator
  ;;;[1 1 1] Calculate Rotation of DmgIndicator
  (Class|Widget|SetRenderTransformAngle (Variables|Default|GetDIndicatorWBP) (.Yaw (Math|Rotator|BreakRotator (Math|Rotator|Delta(Rotator) (Math|Rotator|FindLookatRotation (Transformation|GetActorLocation) (stale Custom|TakeDamage WorldLoc)) (Transformation|GetActorRotation))))))

(event Custom|GameOver
  (bind _returnvalue (Game|GetPlayerController 0))
  ;[1 1 1] GameOverMenu
  (Game|SetGamePaused true)
  (bind _returnvalue_2 (UserInterface|CreateWidget "/Game/Menus/WBP_GameOVer.WBP_GameOVer_C" _returnvalue))
  (UserInterface|Viewport|AddtoViewport _returnvalue_2 0)
  (Variables|/Script/Engine.PlayerController|SetbShowMouseCursor _returnvalue true))

(event Custom|RestartIndicTimer
  (bind _dindicatorwbp (Variables|Default|GetDIndicatorWBP))
  ;[0.07573 0.3843 1] TakeDamage
  ;;[0.2423 0.116 1] DmgIndicator
  ;;;[1 1 1] Ensure widget lasts the same time per target
  (Utilities|FlowControl|RetriggerableDelay 1.25)
  (UserInterface|Animation|PlayAnimation _dindicatorwbp (Variables|/Game/CharacterBP/HUD/Images/WBP_DamageIndicator.WBP_DamageIndicator_C|GetfadeOut _dindicatorwbp) 0.0 1 "Forward" 1.0)
  (Utilities|FlowControl|Delay 0.5)
  (Widget|RemovefromParent (Variables|Default|GetDIndicatorWBP))
  (Utilities|Time|ClearandInvalidateTimerbyHandle (stale Custom|TakeDamage _returnvalue)))

(event Custom|Resume
  (bind _returnvalue (Game|GetPlayerController 0))
  ;[1 1 1] Resume Game
  (Game|SetGamePaused false)
  (Widget|RemovefromParent (Variables|Default|GetPauseMenuRef))
  (Input|SetInputModeGameOnly _returnvalue)
  (Variables|/Script/Engine.PlayerController|SetbShowMouseCursor _returnvalue false))

(event EventBeginPlay
  ;[1 1 1] Initialize
  (Utilities|FlowControl|Sequence
    (:then_0
      (CallFunction|ModifyMovement))
    (:then_1
      (bind _returnvalue (UserInterface|CreateWidget "/Game/CharacterBP/HUD/WBP_Crosshair.WBP_Crosshair_C"))
      (Variables|Default|SetCrosshairWBP _returnvalue)
      (bind _returnvalue_2 (UserInterface|CreateWidget "/Game/CharacterBP/HUD/WBP_TakeDmg.WBP_TakeDmg_C"))
      (bind _output_get (Variables|Default|SetBloodWBP _returnvalue_2))
      (Widget|SetRenderOpacity _output_get 0.0)
      (UserInterface|Viewport|AddtoViewport _output_get 0)
      (bind _returnvalue_3 (UserInterface|CreateWidget "/Game/CharacterBP/HUD/WBP_Player.WBP_Player_C"))
      (UserInterface|Viewport|AddtoViewport _returnvalue_3 0)
      (bind _returnvalue_4 (UserInterface|CreateWidget "/Game/CharacterBP/HUD/WBP_EnergyBar.WBP_EnergyBar_C"))
      (Variables|Default|SetEnergyWBP _returnvalue_4)
      (bind _returnvalue_5 (UserInterface|CreateWidget "/Game/CharacterBP/HUD/Images/WBP_DamageIndicator.WBP_DamageIndicator_C"))
      (Variables|Default|SetDIndicatorWBP _returnvalue_5)
      (Input|SetInputModeGameOnly (Game|GetPlayerController 0))
      (Variables|Default|SetCanActiveAgain true))
    (:then_2
      (Variables|Default|SetinRifleStance true)
      (Variables|Default|SetcanSwitchWeapon true))
    (:then_3
      (CallFunction|AttachWeapon "/Game/CharacterBP/Weapons/BP_Rifle.BP_Rifle_C"))
    (:then_4
      (CallFunction|ClampCamera 5e+01 -4e+01))))

(event Collision|EventActorBeginOverlap
  (params (OtherActor :type Actor%20Object%20Reference)))

(event Game|Damage|EventAnyDamage
  (params (Damage :type Float%20%28single-precision%29) (DamageType :type Damage%20Type%20Object%20Reference) (InstigatedBy :type Controller%20Object%20Reference) (DamageCauser :type Actor%20Object%20Reference))
  (Development|PrintString "Hello"))

(event EventTick
  (params (DeltaSeconds :type Float%20%28single-precision%29))
  ;[1 1 1] ActiveBlockShield
  (if (not (Variables|Default|GetCanActiveAgain))
    (Utilities|FlowControl|Delay 6e+01)
    (Variables|Default|SetCanActiveAgain true)))

(event Input|ActionEvents|InputActionReloadWeapon
  (params (Key :type Key%20Structure :default "None"))
  ;[0 1 0.04499] Attack
  (:Pressed
    (Default|ReloadWeapon (Variables|Default|GetCurrentWeapon))))

(event Input|ActionEvents|InputActionAim
  (params (Key :type Key%20Structure :default "None"))
  ;[1 1 1] Aiming / Field of View
  (:Pressed
    (if (Variables|Default|GetisSprinting)
      (Variables|Default|SetisSprinting false))
    (Variables|Default|SetisAiming true)
    (CallFunction|ModifyMovement)
    (CallFunction|ClampCamera 3e+01 -75.0)
    (UserInterface|Viewport|AddtoViewport (Variables|Default|GetCrosshairWBP) 0)
    (bind _fieldofview (Timeline|Timeline_0 Play)
      (:Update
        (Camera|SetFieldOfView (Variables|Default|GetCamera) _fieldofview))))
  (:Released
    (Variables|Default|SetisAiming false)
    (CallFunction|ModifyMovement)
    (CallFunction|ClampCamera 5e+01 -4e+01)
    (Widget|RemovefromParent (Variables|Default|GetCrosshairWBP))
    (Timeline|Timeline_0 Reverse)))

(event Input|ActionEvents|InputActionActiveBlockField
  (params (Key :type Key%20Structure :default "None"))
  (bind _mesh (Variables|Character|GetMesh))
  (bind _relativelocation (Variables|/Script/Engine.SceneComponent|GetRelativeLocation _mesh))
  (bind (_x _y _z) (Math|Vector|BreakVector _relativelocation))
  ;[1 1 1] ActiveBlockShield
  (:Pressed
    (if (Variables|Default|GetCanActiveAgain)
      (Effects|SpawnEmitterAttached "/Game/BlockField/PS_BlockField.PS_BlockField" _mesh "None" (Math|Vector|MakeVector _x _y (+ _z 1.8e+02)))
      (Variables|Default|SetIsBlockFieldActived true)
      (Variables|Default|SetCanActiveAgain false)
      (Utilities|FlowControl|Delay 1e+01)
      (Variables|Default|SetIsBlockFieldActived false))))

(event Input|ActionEvents|InputActionSprint
  (params (Key :type Key%20Structure :default "None"))
  ;[1 1 1] Sprint
  (:Pressed
    (Variables|Default|SetcanSwitchWeapon false)
    (if true
      (Widget|RemovefromParent (Variables|Default|GetCrosshairWBP)))
    (Variables|Default|SetisSprinting true)
    (CallFunction|ModifyMovement))
  (:Released
    (Variables|Default|SetcanSwitchWeapon true)
    (if (Variables|Default|GetisAiming)
      (if (UserInterface|Viewport|IsinViewport (Variables|Default|GetCrosshairWBP))
        _
        (else
          (UserInterface|Viewport|AddtoViewport (Variables|Default|GetCrosshairWBP) 0))))
    (Variables|Default|SetisSprinting false)
    (CallFunction|ModifyMovement)))

(event Input|ActionEvents|InputActionEquipWeapon3
  (params (Key :type Key%20Structure :default "None"))
  ;[1 1 1] Switch Weapons
  (:Pressed
    (if (Variables|Default|GetcanSwitchWeapon)
      (Variables|Default|SetinRifleStance true)
      (Variables|Default|SetInPistolStance false)
      (Variables|Default|SetinMeleeStance false)
      (CallFunction|ReplaceWeapon "/Game/CharacterBP/Weapons/BP_OrbGun.BP_OrbGun_C" (Variables|Default|GetorbClip)))))

(event Input|ActionEvents|InputActionEquipWeapon2
  (params (Key :type Key%20Structure :default "None"))
  ;[1 1 1] Switch Weapons
  (:Pressed
    (if (Variables|Default|GetcanSwitchWeapon)
      (Variables|Default|SetInPistolStance true)
      (Variables|Default|SetinRifleStance false)
      (Variables|Default|SetinMeleeStance false)
      (CallFunction|ReplaceWeapon "/Game/CharacterBP/Weapons/BP_Pistol.BP_Pistol_C" (Variables|Default|GetpistolClip)))))

(event Input|ActionEvents|InputActionEquipWeapon1
  (params (Key :type Key%20Structure :default "None"))
  ;[1 1 1] Switch Weapons
  (:Pressed
    (if (Variables|Default|GetcanSwitchWeapon)
      (Variables|Default|SetinRifleStance true)
      (Variables|Default|SetInPistolStance false)
      (Variables|Default|SetinMeleeStance false)
      (CallFunction|ReplaceWeapon "/Game/CharacterBP/Weapons/BP_Rifle.BP_Rifle_C" (Variables|Default|GetrifleClip)))))

(event Input|ActionEvents|InputActionFireWeapon
  (params (Key :type Key%20Structure :default "None"))
  (bind _currentweapon (Variables|Default|GetCurrentWeapon))
  ;[0 1 0.04499] Attack
  (:Pressed
    (if (Variables|Default|GetinMeleeStance)
      (Default|FireWeapon _currentweapon :!label _label)
      (else
        (bind _return (CallFunction|CanIShoot))
        (if _return
          (goto _label)))))
  (:Released
    (Default|StopFiring _currentweapon)))

(event Input|ActionEvents|InputActionEquipWeapon4
  (params (Key :type Key%20Structure :default "None"))
  ;[1 1 1] Switch Weapons
  (:Pressed
    (if (Variables|Default|GetcanSwitchWeapon)
      (Variables|Default|SetinMeleeStance true)
      (Variables|Default|SetinRifleStance false)
      (Variables|Default|SetInPistolStance false)
      (CallFunction|ReplaceWeapon "/Game/CharacterBP/Weapons/Melee/BP_Sword.BP_Sword_C" (Variables|Default|GetrailClip)))))

(event Input|ActionEvents|InputActionShieldBomb
  (params (Key :type Key%20Structure :default "None"))
  ;[0 1 0.04499] Attack
  ;;[0 1 0.3215] EnergySlam
  (:Pressed
    (if (>= (Variables|Default|GetcurrentShield) (/ (Variables|Default|GetmaxShield) 2.0))
      (Variables|Default|SetenergyBombDmg (Variables|Default|GetcurrentShield))
      (Variables|Default|SetcurrentShield 0.0)
      (Animation|Montage|PlayMontage (Variables|Character|GetMesh) "/Game/CharacterBP/Animation/Animations/Misc/AM_EnergySlam_Character.AM_EnergySlam_Character"
        (:then
          (Utilities|Time|ClearandInvalidateTimerbyHandle (Variables|Default|GetEnergyTimer))
          (Variables|Default|SetshieldActivated false)
          (Variables|Default|SetcanShoot false)
          (Utilities|FlowControl|Delay 25.5)
          (Variables|Default|SetshieldActivated true)
          (CallFunction|Restoreshield))
        (:OnCompleted
          (Variables|Default|SetcanShoot true :!label _label))
        (:OnInterrupted
          (goto _label))))))

(event Input|ActionEvents|InputActionSlowTime
  (params (Key :type Key%20Structure :default "None"))
  (bind _bprifleref (Variables|Default|GetbpRifleRef))
  ;[1 1 1] Slow Time
  (:Pressed
    ;;[1 1 1] Do A then B
    (Utilities|FlowControl|FlipFlop
      (:A
        (Variables|Default|SetisSlowtimeOn true)
        (Variables|Default|SetcurrentHP (- (Variables|Default|GetcurrentHP) 3e+01))
        (CallFunction|SetBloodAlpha)
        (Utilities|Time|SetGlobalTimeDilation 0.1)
        (Variables|/Script/Engine.Actor|SetCustomTimeDilation (Game|Player|GetPlayerPawn 0) 1e+01)
        (Variables|/Game/CharacterBP/Weapons/BP_Weapon_Parent.BP_Weapon_Parent_C|SetfiringRate _bprifleref 0.0123)
        ;[1 1 1] Slowtime Effect
        (bind _returnvalue (Utilities|Time|SetTimerbyEvent (delegate Custom|SlowEffect) 0.05 true))
        (Variables|Default|SetSlowTimeTimer _returnvalue))
      (:B
        (Variables|Default|SetisSlowtimeOn false)
        (Utilities|Time|SetGlobalTimeDilation 1.0)
        (Variables|/Script/Engine.Actor|SetCustomTimeDilation (Game|Player|GetPlayerPawn 0) 1.0)
        (Variables|/Game/CharacterBP/Weapons/BP_Weapon_Parent.BP_Weapon_Parent_C|SetfiringRate _bprifleref 0.123)
        (Utilities|Time|ClearandInvalidateTimerbyHandle (Variables|Default|GetSlowTimeTimer))))))

(event Input|AxisEvents|InputAxisMoveForward
  (params (AxisValue :type Float%20%28single-precision%29))
  ;[1 1 1] Character Controller
  (Pawn|Input|AddMovementInput (Math|Vector|GetForwardVector (Pawn|GetControlRotation :!class /Script/Engine.Pawn)) AxisValue false))

(event Input|AxisEvents|InputAxisMoveRight
  (params (AxisValue :type Float%20%28single-precision%29))
  ;[1 1 1] Character Controller
  (Pawn|Input|AddMovementInput (Math|Vector|GetRightVector (Pawn|GetControlRotation :!class /Script/Engine.Pawn)) AxisValue false))

(event Input|AxisEvents|InputAxisTurn
  (params (AxisValue :type Float%20%28single-precision%29))
  ;[1 1 1] Character Controller
  (Pawn|Input|AddControllerYawInput AxisValue))

(event Input|AxisEvents|InputAxisLookUp
  (params (AxisValue :type Float%20%28single-precision%29))
  ;[1 1 1] Character Controller
  (Pawn|Input|AddControllerPitchInput AxisValue))

(event Input|KeyboardEvents|Q
  (params (Key :type Key%20Structure :default "None"))
  (bind _bloodwbp (Variables|Default|GetBloodWBP))
  ;[0 1 0.04499] Attack
  ;;[1 1 1] Blood splat
  (:Pressed
    ;;;[1 1 1] Debug blood splat
    (Utilities|FlowControl|FlipFlop
      (:A
        (Widget|RemovefromParent _bloodwbp)
        (Development|PrintString "Hiding bloodscreen"))
      (:B
        (UserInterface|Viewport|AddtoViewport _bloodwbp 0)
        (Development|PrintString "Showing bloodscreen")))))

(event Input|KeyboardEvents|SpaceBar
  (params (Key :type Key%20Structure :default "None"))
  (bind _teleportcomponent (Variables|Default|GetTeleportComponent))
  ;[1 1 1] Prototype teleport mechanic
  (:Pressed
    (Transformation|Teleport (Transformation|GetWorldLocation _teleportcomponent) (Transformation|GetWorldRotation _teleportcomponent))))

(event Input|KeyboardEvents|P
  (params (Key :type Key%20Structure :default "None"))
  (bind _returnvalue (Game|GetPlayerController 0))
  ;[1 1 1] Activate Pause Menu
  (:Pressed
    (Game|SetGamePaused true)
    (Utilities|IsValid (Variables|Default|GetPauseMenuRef)
      (:Is%20Valid
        _)
      (:Is%20Not%20Valid
        (bind _returnvalue_2 (UserInterface|CreateWidget "/Game/Menus/WBP_PauseMenu.WBP_PauseMenu_C" _returnvalue))
        (bind _output_get (Variables|Default|SetPauseMenuRef _returnvalue_2))))
    (UserInterface|Viewport|AddtoViewport _output_get 0)
    (Input|SetInputModeUIOnly _returnvalue (Variables|Default|GetPauseMenuRef) "DoNotLock")
    (Variables|/Script/Engine.PlayerController|SetbShowMouseCursor _returnvalue true)))

(fn ConstructionScript)

(fn ModifyMovement
  (bind _charactermovement (Variables|Character|GetCharacterMovement))
  (if (Variables|Default|GetisSprinting)
    ;[1 1 1] Run Speed
    (Variables|/Script/Engine.CharacterMovementComponent|SetMaxWalkSpeed _charactermovement 6e+02)
    (elif (Variables|Default|GetisAiming)
      ;[1 1 1] Aim Speed
      (Variables|/Script/Engine.CharacterMovementComponent|SetMaxWalkSpeed _charactermovement 175.0)
      (else
        ;[1 1 1] Walk Speed
        (Variables|/Script/Engine.CharacterMovementComponent|SetMaxWalkSpeed _charactermovement 2.5e+02)))))

(fn AttachWeapon
  (params (Weapon :type Actor%20Class%20Reference))
  ;[1 1 1] Attach Weapon
  (bind _returnvalue (Game|SpawnActorfromClass (Variables|Default|GetDesiredWeapon) (Transformation|GetActorTransform) "AlwaysSpawn" 0 0))
  (bind _asbp_weapon_parent (Utilities|Casting|CastToBP_Weapon_Parent _returnvalue))
  (bind _output_get (Variables|Default|SetCurrentWeapon _asbp_weapon_parent))
  (Transformation|AttachComponentToComponent _output_get (Variables|Character|GetMesh) "WeaponSocket" "SnapToTarget" "SnapToTarget" "KeepWorld" true)
  (Default|SetCamera _asbp_weapon_parent (Variables|Default|GetCamera)))

(fn ClampCamera
  (params (PitchMax :type Float%20%28single-precision%29) (PitchMin :type Float%20%28single-precision%29))
  (bind _returnvalue (Game|GetPlayerCameraManager 0))
  (Variables|/Script/Engine.PlayerCameraManager|SetViewPitchMax _returnvalue PitchMax)
  (Variables|/Script/Engine.PlayerCameraManager|SetViewPitchMin _returnvalue PitchMin))

(fn ReplaceWeapon
  (params (Weapon :type Actor%20Class%20Reference) (AmmoType :type Integer))
  (bind _energywbp (Variables|Default|GetEnergyWBP))
  ;[1 1 1] Attach Weapon
  (Actor|DestroyActor (Variables|Default|GetCurrentWeapon))
  (bind _returnvalue (Game|SpawnActorfromClass Weapon (Transformation|GetActorTransform) "AlwaysSpawn" 0 0))
  (bind _asbp_weapon_parent (Utilities|Casting|CastToBP_Weapon_Parent _returnvalue))
  (bind _output_get (Variables|Default|SetCurrentWeapon _asbp_weapon_parent))
  (Variables|/Game/CharacterBP/Weapons/BP_Weapon_Parent.BP_Weapon_Parent_C|SetCurrentAmmo _output_get AmmoType)
  (Transformation|AttachComponentToComponent _output_get (Variables|Character|GetMesh) "WeaponSocket" "SnapToTarget" "SnapToTarget" "KeepWorld" true)
  (Default|SetCamera _asbp_weapon_parent (Variables|Default|GetCamera))
  (if (UserInterface|Viewport|IsinViewport _energywbp)
    (Widget|RemovefromParent _energywbp)))

(fn UpdateStance)

(fn CanIShoot
  (return (Math|Boolean|ANDBoolean (Variables|Default|GetisAiming) (Variables|Default|GetcanShoot) (Variables|Default|GetcanSwitchWeapon))))

(fn AddKill
  (Math|Integer|IncrementInt (Variables|Default|GetkillCount)
    (:%20%20
      (Development|PrintString (Utilities|String|ToString(Integer) (Variables|Default|GetkillCount))))))