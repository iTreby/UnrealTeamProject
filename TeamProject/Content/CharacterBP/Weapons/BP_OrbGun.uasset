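; BP_OrbGun is a chargeable weapon that fires an orb on release, sized by the built-up charge.
; FireWeapon starts a looping ChargeWeapon timer that raises ChargeMeter to a cap while not sprinting, spawning scaled muzzle flashes and showing the character's energy widget.
; StopFiring above a minimum charge sets projectile scale, spends OrbClip ammo, shakes the camera and calls the parent's FireWeapon.
; ReloadWeapon refills the character's OrbClip.
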(event Custom|ChargeWeapon
  ;[1 1 1] Override Fire
  (if (Math|Boolean|ANDBoolean (< (Variables|Default|GetchargeMeter) 6.0) (Variables|Default|GetisFiring) (not (Variables|/Game/CharacterBP/BP_Character.BP_Character_C|GetisSprinting (Variables|Default|GetCharRef))))
    (bind _output_get (Variables|Default|SetchargeMeter (+ (Variables|Default|GetchargeMeter) (Variables|Default|GetchargeRate))))
    (Variables|/Game/CharacterBP/BP_Character.BP_Character_C|SetchargeMeter (Variables|Default|GetCharRef) _output_get)
    (bind _output_get_2 (Variables|Default|Setscale (* (Math|Conversions|ToVector(Float) (Variables|Default|GetchargeMeter)) 0.175)))
    (Effects|SpawnEmitterAttached "/Game/CharacterBP/Weapons/Gun_Meshes/SciFiWeapDark/FX/Particles/P_AssaultRifle_MuzzleFlash_Light.P_AssaultRifle_MuzzleFlash_Light" (Variables|Default|GetWeaponMesh) "Muzzle" "0, 0, 0" "0, 0, 0" _output_get_2)
    (if (not (Variables|Default|GetenergyShown))
      (Variables|Default|SetenergyShown true)
      (Audio|PlaySound2D "/Game/CharacterBP/Weapons/Gun_Meshes/SciFiWeapLight/Sound/Shotgun/Wavs/Shotgun_ReloadOut02.Shotgun_ReloadOut02" 1.0 1.0 0.0 0 0)
      (UserInterface|Viewport|AddtoViewport (Variables|/Game/CharacterBP/BP_Character.BP_Character_C|GetEnergyWBP (Variables|Default|GetCharRef)) 0))
    (else
      (Variables|Default|SetfullyCharged true))))

(event EventBeginPlay
  (Components|Activation|Deactivate (Variables|Default|GetParticleSystem))
  (|CallParentFunction))

(event Collision|EventActorBeginOverlap
  (params (OtherActor :type Actor%20Object%20Reference))
  (|CallParentFunction OtherActor) ; This node is disabled and will not be called.\nDrag off pins to build functionality.
)

(event EventTick
  (params (DeltaSeconds :type Float%20%28single-precision%29))
  (|CallParentFunction DeltaSeconds))

(event EventReloadWeapon
  ;[1 1 1] Reload
  (Variables|/Game/CharacterBP/BP_Character.BP_Character_C|SetorbClip (Variables|Default|GetCharRef) (Variables|Default|GetMaxAmmo))
  (|CallParentFunction))

(event EventStopFiring
  (bind _charref (Variables|Default|GetCharRef))
  ;[1 1 1] Release Fire
  (if (Variables|Default|GetisFiring)
    (Variables|Default|SetisFiring false)
    (if (>= (Variables|Default|GetchargeMeter) 1.0)
      (Variables|Default|Setscale (* (Math|Conversions|ToVector(Float) (Variables|Default|GetchargeMeter)) 9.0))
      (Variables|Default|SetchargeMeter 0.0)
      (Utilities|Time|ClearandInvalidateTimerbyHandle (Variables|Default|GetTimer))
      ;;[1 1 1] Remove Energy WBP
      (Widget|RemovefromParent (Variables|/Game/CharacterBP/BP_Character.BP_Character_C|GetEnergyWBP (Variables|Default|GetCharRef)))
      (Variables|Default|SetenergyShown false)
      (Variables|/Game/CharacterBP/BP_Character.BP_Character_C|SetorbClip _charref (- (Variables|/Game/CharacterBP/BP_Character.BP_Character_C|GetorbClip _charref) 1))
      (Camera|PlayWorldCameraShake "/Game/CharacterBP/BP_CamShake.BP_CamShake_C" (Transformation|GetActorLocation _charref) 0.0 5e+02)
      (|CallParentFunction)
      (else
        ;;[1 1 1] Don't shoot below min threshhold
        (Variables|Default|SetchargeMeter 0.0)))))

(event EventFireWeapon
  ;[1 1 1] Override Fire
  (if (> (Variables|/Game/CharacterBP/BP_Character.BP_Character_C|GetorbClip (Variables|Default|GetCharRef)) 0)
    (Variables|Default|SetisFiring true)
    (CallFunction|ChargeWeapon)
    (bind _returnvalue (Utilities|Time|SetTimerbyEvent (delegate Custom|ChargeWeapon) (Variables|Default|GetfiringRate) true))
    (Variables|Default|SetTimer _returnvalue)
    (else
      (Audio|PlaySound2D "/Game/CharacterBP/Weapons/Gun_Meshes/SciFiWeapLight/Sound/GrenadeLauncher/GL_ReloadClick_Cue.GL_ReloadClick_Cue" 1.0 1.0 0.0 0 0))))

(fn ConstructionScript
  (|CallParentFunction))