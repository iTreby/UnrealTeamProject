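; Pistol weapon Blueprint that extends a parent weapon with a nine-round magazine and its own projectile class.
; Firing is blocked during reload or on an empty clip, and decrements the character's PistolClip before calling the parent fire logic.
; Reload checks CurrentAmmo against MaxAmmo, plays a sped-up montage and sound, then refills PistolClip when the montage completes and calls the parent reload.
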(event EventBeginPlay
  (|CallParentFunction)
  (Variables|Default|SetProjectileClass "/Game/CharacterBP/Weapons/Projectiles/BP_Projectile_Pistol.BP_Projectile_Pistol_C")
  (Variables|Default|SetMaxAmmo 9)
  (Variables|Default|SetCurrentAmmo 9))

(event Collision|EventActorBeginOverlap
  (params (OtherActor :type Actor%20Object%20Reference))
  (|CallParentFunction OtherActor) ; This node is disabled and will not be called.\nDrag off pins to build functionality.
)

(event EventTick
  (params (DeltaSeconds :type Float%20%28single-precision%29))
  (|CallParentFunction DeltaSeconds))

(event EventReloadWeapon
  ;[1 1 1] Reload
  (if (!= (Variables|Default|GetCurrentAmmo) (Variables|Default|GetMaxAmmo))
    (Animation|Montage|PlayMontage (Variables|/Script/Engine.Character|GetMesh (Variables|Default|GetCharRef)) "/Game/CharacterBP/Animation/Animations/Pistol/Actions/AM_Reload_Pistol.AM_Reload_Pistol" 1.5
      (:then
        (Audio|PlaySound2D "/Game/CharacterBP/Weapons/Meshes/SciFiWeapLight/Sound/Pistol/Wavs/Pistol_Reload01.Pistol_Reload01" 1.0 1.0 0.0 0 0)
        (Variables|Default|SetisReloading true))
      (:OnCompleted
        (Variables|Default|SetisReloading false)
        (Variables|/Game/CharacterBP/BP_Character.BP_Character_C|SetpistolClip (Variables|Default|GetCharRef) 9)
        (|CallParentFunction)))))

(event EventStopFiring
  (|CallParentFunction))

(event EventFireWeapon
  (bind _charref (Variables|Default|GetCharRef))
  (if (not (Variables|Default|GetisReloading))
    (if (> (Variables|/Game/CharacterBP/BP_Character.BP_Character_C|GetpistolClip _charref) 0)
      (Variables|/Game/CharacterBP/BP_Character.BP_Character_C|SetpistolClip _charref (- (Variables|/Game/CharacterBP/BP_Character.BP_Character_C|GetpistolClip _charref) 1))
      (|CallParentFunction))))

(fn ConstructionScript
  (|CallParentFunction))