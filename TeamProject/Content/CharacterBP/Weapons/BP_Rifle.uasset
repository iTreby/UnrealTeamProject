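; Automatic rifle weapon Blueprint that overrides the parent weapon's fire and reload events.
; FireWeapon fires at once and starts a looping timer at FiringRate, which StopFiring clears.
; Each shot requires active firing, no reload in progress and rounds in the character's RifleClip, which it decrements before calling the parent fire logic.
; Reload refills that character-held clip to MaxAmmo, then calls the parent reload.
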(event Custom|AutomaticFire
  (bind _charref (Variables|Default|GetCharRef))
  ;[1 1 1] Override Fire
  (if (Variables|Default|GetisFiring)
    (if (not (Variables|Default|GetisReloading))
      (if (> (Variables|/Game/CharacterBP/BP_Character.BP_Character_C|GetrifleClip _charref) 0)
        (Variables|/Game/CharacterBP/BP_Character.BP_Character_C|SetrifleClip _charref (- (Variables|/Game/CharacterBP/BP_Character.BP_Character_C|GetrifleClip _charref) 1))
        (|CallParentFunction)))))

(event EventBeginPlay
  (|CallParentFunction)
  (Variables|Default|SetMaxAmmo 32)
  (Variables|Default|SetCurrentAmmo 32))

(event Collision|EventActorBeginOverlap
  (params (OtherActor :type Actor%20Object%20Reference))
  (|CallParentFunction OtherActor) ; This node is disabled and will not be called.\nDrag off pins to build functionality.
)

(event EventTick
  (params (DeltaSeconds :type Float%20%28single-precision%29))
  (|CallParentFunction DeltaSeconds))

(event EventReloadWeapon
  ;[1 1 1] Reload
  (Variables|/Game/CharacterBP/BP_Character.BP_Character_C|SetrifleClip (Variables|Default|GetCharRef) (Variables|Default|GetMaxAmmo))
  (|CallParentFunction))

(event EventStopFiring
  ;[1 1 1] Override Fire
  (Variables|Default|SetisFiring false)
  (Utilities|Time|ClearandInvalidateTimerbyHandle (Variables|Default|GetTimer)))

(event EventFireWeapon
  ;[1 1 1] Override Fire
  (Variables|Default|SetisFiring true)
  (CallFunction|AutomaticFire)
  (bind _returnvalue (Utilities|Time|SetTimerbyEvent (delegate Custom|AutomaticFire) (Variables|Default|GetfiringRate) true))
  (Variables|Default|SetTimer _returnvalue))

(fn ConstructionScript
  (|CallParentFunction))