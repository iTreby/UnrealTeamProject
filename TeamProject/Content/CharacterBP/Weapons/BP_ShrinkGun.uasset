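; BP_ShrinkGun is an automatic-fire weapon that spawns projectiles, presumably with a shrink effect given its name.
; Its FireWeapon override fires immediately and starts a looping timer at FiringRate, which StopFiring clears.
; While ammo remains, each shot plays the looping fire animation, spawns ProjectileClass at the CalcShootInfo transform and decrements CurrentAmmo.
; The gun itself holds no shrink logic, only a debug print.
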(event Custom|ShootLaser
  ;[1 1 1] FireWeapon (Override)
  (if (> (Variables|Default|GetCurrentAmmo) 0)
    (Components|Animation|PlayAnimation (Variables|Default|GetWeaponMesh) (Variables|Default|GetFireAnim) true)
    (bind _projectilespawninfo (CallFunction|CalcShootInfo))
    (Game|SpawnActorfromClass (Variables|Default|GetProjectileClass) _projectilespawninfo "Undefined" 0 0)
    (Variables|Default|SetCurrentAmmo (- (Variables|Default|GetCurrentAmmo) 1))))

(event Custom|AutomaticFire
  ;[1 1 1] FireWeapon (Override)
  (if (Variables|Default|GetisFiring)
    (CallFunction|ShootLaser)
    (Development|PrintString "calling shrink")))

(event EventBeginPlay
  (|CallParentFunction) ; This node is disabled and will not be called.\nDrag off pins to build functionality.
)

(event Collision|EventActorBeginOverlap
  (params (OtherActor :type Actor%20Object%20Reference))
  (|CallParentFunction OtherActor) ; This node is disabled and will not be called.\nDrag off pins to build functionality.
)

(event EventTick
  (params (DeltaSeconds :type Float%20%28single-precision%29))
  (|CallParentFunction DeltaSeconds) ; This node is disabled and will not be called.\nDrag off pins to build functionality.
)

(event EventFireWeapon
  ;[1 1 1] FireWeapon (Override)
  (Variables|Default|SetisFiring true)
  (bind _returnvalue (Utilities|Time|SetTimerbyEvent (delegate Custom|AutomaticFire) (Variables|Default|GetfiringRate) true))
  (CallFunction|AutomaticFire))

(event EventStopFiring
  ;[1 1 1] FireWeapon (Override)
  (Utilities|Time|ClearandInvalidateTimerbyHandle (stale EventFireWeapon _returnvalue))
  (Variables|Default|SetisFiring false))

(fn ConstructionScript
  (|CallParentFunction))