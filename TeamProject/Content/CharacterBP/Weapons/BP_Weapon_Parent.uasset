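; Base weapon Blueprint for the player character, providing projectile firing and reloading with ammo tracking.
; FireWeapon plays the mesh animation, spawns a projectile and spends one round.
; CalcShootInfo traces from the camera supplied through SetCamera, then aims the muzzle transform at the impact or trace end so shots converge on screen center.
; ReloadWeapon plays a character montage and sound, mirrors IsReloading onto BP_Character and refills ammo on completion, without a reserve pool.
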(event Custom|StopFiring)

(event Custom|FireWeapon
  ;[1 1 1] Fire Weapon
  (if (> (Variables|Default|GetCurrentAmmo) 0)
    (Components|Animation|PlayAnimation (Variables|Default|GetWeaponMesh) (Variables|Default|GetFireAnim) false)
    (bind _projectilespawninfo (CallFunction|CalcShootInfo))
    (Game|SpawnActorfromClass (Variables|Default|GetProjectileClass) _projectilespawninfo "Undefined" 0 0)
    (Variables|Default|SetCurrentAmmo (- (Variables|Default|GetCurrentAmmo) 1))))

(event Custom|ReloadWeapon
  (bind _charref (Variables|Default|GetCharRef))
  ;[1 1 1] Reload
  (if (!= (Variables|Default|GetCurrentAmmo) (Variables|Default|GetMaxAmmo))
    (if (not (Variables|Default|GetisReloading))
      (Animation|Montage|PlayMontage (Variables|/Script/Engine.Character|GetMesh (Variables|Default|GetCharRef)) (Variables|Default|GetReloadAnim) 1.275
        (:then
          (Audio|PlaySound2D (Variables|Default|GetReloadSound) 1.0 1.0 0.0 0 0)
          (Variables|Default|SetisReloading true)
          (Variables|/Game/CharacterBP/BP_Character.BP_Character_C|SetisReloading _charref true))
        (:OnCompleted
          (Variables|Default|SetisReloading false)
          (Variables|/Game/CharacterBP/BP_Character.BP_Character_C|SetisReloading _charref false)
          (if (> (Variables|Default|GetMaxAmmo) 0)
            (Variables|Default|SetCurrentAmmo (Variables|Default|GetMaxAmmo))))))))

(event EventBeginPlay
  ;[1 1 1] Reference
  (bind _asbp_character (Utilities|Casting|CastToBP_Character (Game|Player|GetPlayerPawn 0)))
  (Variables|Default|SetCharRef _asbp_character))

(event Collision|EventActorBeginOverlap
  (params (OtherActor :type Actor%20Object%20Reference)))

(event EventTick
  (params (DeltaSeconds :type Float%20%28single-precision%29)))

(fn ConstructionScript)

(fn CalcShootInfo
  (bind _weaponmesh (Variables|Default|GetWeaponMesh))
  (bind _playercam (Variables|Default|GetPlayerCam))
  (bind _returnvalue (Transformation|GetWorldLocation _playercam))
  (bind _returnvalue_2 (Math|Vector|GetForwardVector _playercam))
  (bind _returnvalue_3 (Transformation|GetSocketLocation _weaponmesh "Muzzle"))
  (bind _returnvalue_4 (* _returnvalue_2 1e+04))
  (bind _returnvalue_5 (+ _returnvalue _returnvalue_4))
  (bind (_outhit _returnvalue_6) (Collision|LineTraceByChannel _returnvalue _returnvalue_5 "TraceTypeQuery3" false 0 "None"))
  (if _returnvalue_6
    (return (Math|Transform|MakeTransform _returnvalue_3 (Math|Rotator|FindLookatRotation _returnvalue_3 (.ImpactPoint (Collision|BreakHitResult _outhit))) (Variables|Default|Getscale)))
    (else
      (return (Math|Transform|MakeTransform _returnvalue_3 (Math|Rotator|FindLookatRotation _returnvalue_3 _returnvalue_5) (Variables|Default|Getscale))))))

(fn SetCamera
  (params (Camera :type Camera%20Component%20Object%20Reference))
  (Variables|Default|SetPlayerCam Camera))