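; Friendly projectile that temporarily turns any overlapped BP_Enemy_Parent friendly.
; On overlap it sets the enemy's Friendly flag, writes the player character and a friendly bool to its AI blackboard, and prints a debug message.
; After a fixed Delay in the same event chain, it clears both keys and the flag, so the revert relies on this actor still existing.
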(event EventBeginPlay
  (|CallParentFunction) ; This node is disabled and will not be called.\nDrag off pins to build functionality.
)

(event EventTick
  (params (DeltaSeconds :type Float%20%28single-precision%29))
  (|CallParentFunction DeltaSeconds) ; This node is disabled and will not be called.\nDrag off pins to build functionality.
)

(event Collision|EventActorBeginOverlap
  (params (OtherActor :type Actor%20Object%20Reference))
  (bind _playerkey (Variables|Default|GetPlayerKey))
  (bind _isfriendlykey (Variables|Default|GetIsFriendlyKey))
  (bind _asbp_enemy_parent (Utilities|Casting|CastToBP_Enemy_Parent OtherActor))
  (Variables|/Game/Enemies/Blueprints/BP_Enemy_Parent.BP_Enemy_Parent_C|SetFriendly _asbp_enemy_parent true)
  (AI|Components|Blackboard|SetValueasObject (AI|GetBlackboard (AI|GetAIController _asbp_enemy_parent)) _playerkey (Game|GetPlayerCharacter 0))
  (bind _output_get (Variables|Default|SetIsFriendly true))
  (AI|Components|Blackboard|SetValueasBool (AI|GetBlackboard (AI|GetAIController _asbp_enemy_parent)) _isfriendlykey _output_get)
  (Development|PrintString "Friendly")
  (Utilities|FlowControl|Delay 15.0)
  (AI|Components|Blackboard|ClearValue (AI|GetBlackboard (AI|GetAIController _asbp_enemy_parent)) _isfriendlykey)
  (AI|Components|Blackboard|ClearValue (AI|GetBlackboard (AI|GetAIController _asbp_enemy_parent)) _playerkey)
  (Variables|/Game/Enemies/Blueprints/BP_Enemy_Parent.BP_Enemy_Parent_C|SetFriendly _asbp_enemy_parent false))

(fn ConstructionScript
  (|CallParentFunction))