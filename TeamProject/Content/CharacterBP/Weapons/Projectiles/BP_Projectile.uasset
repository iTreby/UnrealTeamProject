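; BP_Projectile is a weapon projectile that damages what its Bullet component hits and expires after four seconds.
; On hit it plays impact effects and sound, then applies randomised damage, destroying itself unless IsOrb is set.
; AddVariance overwrites Damage with each roll, so variance accumulates over repeated orb hits.
; An unconnected draft of a mine upgrade would spawn a HealthPack for orbs.
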(event OnComponentHit(Bullet)
  (params (HitComponent :type Primitive%20Component%20Object%20Reference) (OtherActor :type Actor%20Object%20Reference) (OtherComp :type Primitive%20Component%20Object%20Reference) (NormalImpulse :type Vector :default "0, 0, 0") (Hit :type Hit%20Result%20Structure%20%28by%20ref%29))
  (bind _impactpoint (Collision|BreakHitResult Hit))
  (Effects|SpawnEmitteratLocation (Variables|Default|GetImpact%20Effect) _impactpoint (Transformation|GetActorRotation))
  (Audio|PlaySoundatLocation (Variables|Default|GetImpact%20Sound) _impactpoint "0, 0, 0" 1.0 1.0 0.0 0 0 0)
  (bind _damage (CallFunction|AddVariance))
  (Game|Damage|ApplyDamage OtherActor _damage 0 self)
  (if (not (Variables|Default|GetisOrb))
    (Actor|DestroyActor)))

(event EventBeginPlay
  (Actor|SetLifeSpan 4.0))

(event Collision|EventActorBeginOverlap
  (params (OtherActor :type Actor%20Object%20Reference)))

(event EventTick
  (params (DeltaSeconds :type Float%20%28single-precision%29)))

(fn ConstructionScript)

(fn AddVariance
  (bind _damagevariance (Variables|Default|GetDamageVariance))
  (Variables|Default|SetDamage (Math|Random|RandomFloatinRange (- (Variables|Default|GetDamage) _damagevariance) (+ (Variables|Default|GetDamage) _damagevariance)))
  (return (Variables|Default|GetDamage)))