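; BP_Projectile_Orb is a charged orb projectile whose damage scales with the player character's ChargeMeter.
; On BeginPlay it casts player 0's character to BP_Character, derives Damage from the charge, prints it and sets a fixed lifespan.
; It then calls the parent BeginPlay and resets the character's ChargeMeter to zero.
; A failed cast skips all of this, including the parent call; no movement or hit logic appears in this graph.
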(event EventBeginPlay
  (bind _asbp_character (Utilities|Casting|CastToBP_Character (Game|GetPlayerCharacter 0)))
  (bind _output_get (Variables|Default|SetCharRef _asbp_character))
  (bind _output_get_2 (Variables|Default|SetDamage (* (Variables|/Game/CharacterBP/BP_Character.BP_Character_C|GetchargeMeter _output_get) 1e+01)))
  (Development|PrintString (Utilities|String|ToString(Float) _output_get_2))
  (Actor|SetLifeSpan 2e+01)
  (|CallParentFunction)
  (Variables|/Game/CharacterBP/BP_Character.BP_Character_C|SetchargeMeter _output_get 0.0))

(event Collision|EventActorBeginOverlap
  (params (OtherActor :type Actor%20Object%20Reference))
  (|CallParentFunction OtherActor) ; This node is disabled and will not be called.\nDrag off pins to build functionality.
)

(event EventTick
  (params (DeltaSeconds :type Float%20%28single-precision%29))
  (|CallParentFunction DeltaSeconds) ; This node is disabled and will not be called.\nDrag off pins to build functionality.
)

(fn ConstructionScript
  (|CallParentFunction))