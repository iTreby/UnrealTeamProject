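; Player character Blueprint that handles movement, look, sprinting and aiming.
; Axis inputs move the character along the control rotation's forward and right vectors and drive controller yaw and pitch.
; Sprint and Aim set state flags and call ModifyMovement, which picks run, aim or walk speed, with sprint taking priority.
; Pressing Aim cancels sprint and plays a timeline that animates camera field of view, reversed on release.
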(event EventBeginPlay
  (CallFunction|ModifyMovement))

(event Collision|EventActorBeginOverlap
  (params (OtherActor :type Actor%20Object%20Reference)))

(event EventTick
  (params (DeltaSeconds :type Float%20%28single-precision%29)))

(event Input|ActionEvents|InputActionSprint
  (params (Key :type Key%20Structure :default "None"))
  ;[1 1 1] Sprint
  (:Pressed
    (Variables|Default|SetisSprinting true)
    (CallFunction|ModifyMovement))
  (:Released
    (Variables|Default|SetisSprinting false)
    (CallFunction|ModifyMovement)))

(event Input|ActionEvents|InputActionAim
  (params (Key :type Key%20Structure :default "None"))
  (:Pressed
    (if (Variables|Default|GetisSprinting)
      (Variables|Default|SetisSprinting false))
    (Variables|Default|SetisAiming true)
    (CallFunction|ModifyMovement)
    (bind _fieldofview (Timeline|Timeline_0 Play)
      (:Update
        (Camera|SetFieldOfView (Variables|Default|GetCamera) _fieldofview))))
  (:Released
    (Variables|Default|SetisAiming false)
    (CallFunction|ModifyMovement)
    (Timeline|Timeline_0 Reverse)))

(event Input|AxisEvents|InputAxisMoveForward
  (params (AxisValue :type Float%20%28single-precision%29))
  ;[1 1 1] Character Controller
  (Pawn|Input|AddMovementInput (Math|Vector|GetForwardVector (Pawn|GetControlRotation :!class /Script/Engine.Pawn)) AxisValue false))

(event Input|AxisEvents|InputAxisMoveRight
  (params (AxisValue :type Float%20%28single-precision%29))
  ;[1 1 1] Character Controller
  (Pawn|Input|AddMovementInput (Math|Vector|GetRightVector (Pawn|GetControlRotation :!class /Script/Engine.Pawn)) AxisValue false))

(event Input|AxisEvents|InputAxisTurn
  (params (AxisValue :type Float%20%28single-precision%29))
  ;[1 1 1] Character Controller
  (Pawn|Input|AddControllerYawInput AxisValue))

(event Input|AxisEvents|InputAxisLookUp
  (params (AxisValue :type Float%20%28single-precision%29))
  ;[1 1 1] Character Controller
  (Pawn|Input|AddControllerPitchInput AxisValue))

(fn ConstructionScript)

(fn ModifyMovement
  (bind _charactermovement (Variables|Character|GetCharacterMovement))
  (if (Variables|Default|GetisSprinting)
    ;[1 1 1] Run Speed
    (Variables|/Script/Engine.CharacterMovementComponent|SetMaxWalkSpeed _charactermovement 6e+02)
    (elif (Variables|Default|GetisAiming)
      ;[1 1 1] Aim Speed
      (Variables|/Script/Engine.CharacterMovementComponent|SetMaxWalkSpeed _charactermovement 175.0)
      (else
        ;[1 1 1] Walk Speed
        (Variables|/Script/Engine.CharacterMovementComponent|SetMaxWalkSpeed _charactermovement 3e+02)))))