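; Parent enemy Blueprint handling health, melee damage, aggro and death.
; A socket-attached headshot box flags projectile hits for double damage, shown as screen-space combat text before death unpossesses the AI and plays an animation.
; AttackBox overlaps damage the player or Captain Ryan, while SetChasing raises run speed and calls the empty Enrage hook.
; A looping timer, started for behavior tree tasks, smoothly yaws the enemy toward its TargetActor.
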(event OnComponentBeginOverlap(HeadShotBox)
  (params (OverlappedComponent :type Primitive%20Component%20Object%20Reference) (OtherActor :type Actor%20Object%20Reference) (OtherComp :type Primitive%20Component%20Object%20Reference) (OtherBodyIndex :type Integer) (bFromSweep :type Boolean) (SweepResult :type Hit%20Result%20Structure%20%28by%20ref%29))
  ;[1 1 1] Check if headshot
  (Utilities|Casting|CastToBP_Projectile OtherActor)
  (if (not (Variables|Default|GetisHeadShot))
    (Variables|Default|SetisHeadShot true)))

(event OnComponentBeginOverlap(AttackBox)
  (params (OverlappedComponent :type Primitive%20Component%20Object%20Reference) (OtherActor :type Actor%20Object%20Reference) (OtherComp :type Primitive%20Component%20Object%20Reference) (OtherBodyIndex :type Integer) (bFromSweep :type Boolean) (SweepResult :type Hit%20Result%20Structure%20%28by%20ref%29))
  ;[1 1 1] AttackBox Overlap
  (CallFunction|DoDamage OtherActor (Variables|Default|GetDamage)))

(event Custom|Enrage)

(event Custom|Death
  (bind _timer (Variables|Default|GetTimer))
  ;[1 1 1] Death Event
  (Components|Animation|PlayAnimation (Variables|Character|GetMesh) (Variables|Default|GetDeathAnim) false)
  (Pawn|UnPossess (Variables|Default|GetAIC))
  (Collision|SetCollisionEnabled (Variables|Collision|GetCapsuleComponent) "NoCollision")
  (Actor|SetLifeSpan 6e+01)
  (Collision|SetCollisionEnabled (Variables|Default|GetAttackBox) "NoCollision")
  (if (Utilities|Time|IsValidTimerHandle _timer)
    (Utilities|Time|ClearandInvalidateTimerbyHandle _timer)))

(event Custom|LookAtPlayer
  ;[1 1 1] Handle Rotation Between attacks(Called by BTTask)
  (bind _returnvalue (Utilities|Time|SetTimerbyEvent (delegate Custom|RotateTick) 0.01 true))
  (Variables|Default|SetTimer _returnvalue))

(event Custom|RotateTick
  ;[1 1 1] Handle Rotation Between attacks(Called by BTTask)
  (Transformation|SetActorRotation (Math|Interpolation|RInterpTo (Transformation|GetActorRotation) (Math|Rotator|MakeRotator 0.0 0.0 (.Yaw (Math|Rotator|BreakRotator (Math|Rotator|FindLookatRotation (Transformation|GetActorLocation) (Transformation|GetActorLocation (Variables|Default|GettargetActor)))))) 0.5 0.225)))

(event Custom|DoDamage
  (params (AttackedActor :type Actor%20Object%20Reference) (SentDamage :type Float%20%28single-precision%29))
  ;[1 1 1] Damage Target
  (if (Actor|ActorHasTag AttackedActor "Player")
    (bind _asbp_character (Utilities|Casting|CastToBP_Character AttackedActor))
    (Default|TakeDamage _asbp_character SentDamage (Transformation|GetActorLocation) self)
    (elif (Actor|ActorHasTag AttackedActor "Ryan")
      (bind _asbp_cpt_ryan (Utilities|Casting|CastToBP_CptRyan AttackedActor))
      (Default|TakeDamage _asbp_cpt_ryan SentDamage self))))

(event Custom|StopRotate
  ;[1 1 1] Handle Rotation Between attacks(Called by BTTask)
  (Utilities|Time|ClearandInvalidateTimerbyHandle (Variables|Default|GetTimer)))

(event EventBeginPlay
  ;[1 1 1] Dynamically Set HeadshotBox Position
  (Transformation|AttachComponentToComponent (Variables|Default|GetHeadShotBox) (Variables|Character|GetMesh) "HeadShotSocket" "KeepRelative" "KeepRelative" "KeepRelative" true)
  (bind _asaicontroller (Utilities|Casting|CastToAIController (Pawn|GetController)))
  (Variables|Default|SetAIC _asaicontroller)
  (bind _asbp_character (Utilities|Casting|CastToBP_Character (Game|GetPlayerCharacter 0)))
  (Variables|Default|SetCharacter _asbp_character)
  (Collision|SetCollisionEnabled (Variables|Default|GetAttackBox) "NoCollision"))

(event EventTick
  (params (DeltaSeconds :type Float%20%28single-precision%29)))

(event Collision|EventHit
  (params (MyComp :type Primitive%20Component%20Object%20Reference) (Other :type Actor%20Object%20Reference) (OtherComp :type Primitive%20Component%20Object%20Reference) (bSelfMoved :type Boolean) (HitLocation :type Vector :default "0, 0, 0") (HitNormal :type Vector :default "0, 0, 0") (NormalImpulse :type Vector :default "0, 0, 0") (Hit :type Hit%20Result%20Structure%20%28by%20ref%29))
  ;[1 1 1] When Shot
  (Utilities|Casting|CastToBP_Projectile Other)
  (Game|Damage|ApplyDamage 0 0.0 0 0)
  (CallFunction|SetChasing))

(event Game|Damage|EventAnyDamage
  (params (Damage :type Float%20%28single-precision%29) (DamageType :type Damage%20Type%20Object%20Reference) (InstigatedBy :type Controller%20Object%20Reference) (DamageCauser :type Actor%20Object%20Reference))
  (bind _returnvalue (* Damage 2.0))
  ;[1 1 1] Take Dmg / Death
  (if (Variables|Default|GetisHeadShot)
    ;;[1 1 1] Multiply dmg if headshot
    (Variables|Default|SetcurrentHealth (- (Variables|Default|GetcurrentHealth) _returnvalue))
    (if (<= (Variables|Default|GetcurrentHealth) 0.0)
      ;;[1 1 1] Death logic
      (if (not (Variables|Default|GetisDead))
        (Variables|Default|SetisDead true)
        (CallFunction|SpawnCombatText _returnvalue)
        (Variables|Default|SetisHeadShot false :!label _label)
        (CallFunction|Death))
      (else
        (CallFunction|SpawnCombatText _returnvalue)
        (Variables|Default|SetisHeadShot false :!label _label_2)))
    (else
      (Variables|Default|SetcurrentHealth (- (Variables|Default|GetcurrentHealth) Damage))
      (if (<= (Variables|Default|GetcurrentHealth) 0.0)
        (if (not (Variables|Default|GetisDead))
          (Variables|Default|SetisDead true)
          (CallFunction|SpawnCombatText Damage)
          (goto _label))
        (else
          (CallFunction|SpawnCombatText Damage)
          (goto _label_2))))))

(fn ConstructionScript)

(fn SpawnCombatText
  (params (Damage :type Float%20%28single-precision%29))
  (bind _returnvalue (UserInterface|CreateWidget "/Game/CharacterBP/HUD/WBP_CombatText.WBP_CombatText_C" 0 (- (.ScreenPosition (Class|GameplayStatics|ProjectWorldtoScreen (Game|GetPlayerController 0) (Transformation|GetActorLocation) false)) (Variables|Default|GetcmbtTxtOffset)) Damage (Variables|Default|GetisHeadShot)))
  (UserInterface|Viewport|AddtoViewport _returnvalue 0))

(fn SetChasing
  (params (ActorRef :type Actor%20Object%20Reference))
  (Utilities|IsValid ActorRef
    (:Is%20Valid
      ;[1 1 1] Aggro enemies in range
      (bind _asbp_enemy_parent (Utilities|Casting|CastToBP_Enemy_Parent ActorRef))
      (if (not (Variables|BP_Enemy_Parent_C|GetisChasing _asbp_enemy_parent))
        (Variables|BP_Enemy_Parent_C|SetisChasing _asbp_enemy_parent true)
        (Variables|/Script/Engine.CharacterMovementComponent|SetMaxWalkSpeed (Variables|/Script/Engine.Character|GetCharacterMovement _asbp_enemy_parent) (Variables|BP_Enemy_Parent_C|GetrunSpeed _asbp_enemy_parent))
        (Development|PrintString "Chasing")
        (CallFunction|Enrage _asbp_enemy_parent)))
    (:Is%20Not%20Valid
      ;[1 1 1] Self Aggro
      (if (not (Variables|Default|GetisChasing))
        (Variables|Default|SetisChasing true)
        (Variables|/Script/Engine.CharacterMovementComponent|SetMaxWalkSpeed (Variables|Character|GetCharacterMovement) (Variables|Default|GetrunSpeed))
        (CallFunction|Enrage)))))