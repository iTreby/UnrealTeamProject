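; Mutant enemy Blueprint that extends a parent enemy with its own animations and an enraged second phase.
; Enrage waits a random delay, flags the AI Blackboard, then plays enrage and slam montages, unpossessing the AI controller during the slam.
; It then raises speed, swaps the attack montage, repossesses and activates fire.
; Slam and enraged-attack hitboxes start without collision, deal damage on overlap, and are disabled again on death.
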(event OnComponentBeginOverlap(E_AttackHitBox)
  (params (OverlappedComponent :type Primitive%20Component%20Object%20Reference) (OtherActor :type Actor%20Object%20Reference) (OtherComp :type Primitive%20Component%20Object%20Reference) (OtherBodyIndex :type Integer) (bFromSweep :type Boolean) (SweepResult :type Hit%20Result%20Structure%20%28by%20ref%29))
  ;[1 1 1] Apply EnragedAttack Explode Damage
  (CallFunction|DoDamage OtherActor (Variables|Default|GetenragedDmg)))

(event OnComponentBeginOverlap(SlamHitBox)
  (params (OverlappedComponent :type Primitive%20Component%20Object%20Reference) (OtherActor :type Actor%20Object%20Reference) (OtherComp :type Primitive%20Component%20Object%20Reference) (OtherBodyIndex :type Integer) (bFromSweep :type Boolean) (SweepResult :type Hit%20Result%20Structure%20%28by%20ref%29))
  ;[1 1 1] Apply Explosion Damage
  (CallFunction|DoDamage OtherActor (Variables|Default|GetslamDamage)))

(event EventBeginPlay
  ;[1 1 1] Init
  (Variables|Default|SetDeathAnim "/Game/Enemies/Blueprints/Mutant/Animations/Anims/Mutant_Dying.Mutant_Dying")
  (Variables|Default|SetAttackAnim "/Game/Enemies/Blueprints/Mutant/Animations/AM_Attack_Mutant.AM_Attack_Mutant")
  (Variables|Default|SetrunSpeed 2.5e+02)
  (|CallParentFunction))

(event Collision|EventActorBeginOverlap
  (params (OtherActor :type Actor%20Object%20Reference))
  (|CallParentFunction OtherActor) ; This node is disabled and will not be called.\nDrag off pins to build functionality.
)

(event EventTick
  (params (DeltaSeconds :type Float%20%28single-precision%29))
  (|CallParentFunction DeltaSeconds) ; This node is disabled and will not be called.\nDrag off pins to build functionality.
)

(event EventEnrage
  (bind _mesh (Variables|Character|GetMesh))
  ;[1 1 1] Mutant Take Damage & Enrage
  (if (not (Variables|Default|Getenraged))
    (Utilities|FlowControl|Delay (Math|Random|RandomFloatinRange 6.5 9.0))
    (Variables|Default|Setenraged true)
    (AI|Components|Blackboard|SetValueasBool (Variables|/Script/AIModule.AIController|GetBlackboard (Variables|Default|GetAIC)) (Variables|Default|GetisEnraged) true)
    (Animation|Montage|PlayMontage _mesh "/Game/Enemies/Blueprints/Mutant/Animations/AM_Mutant_Enrage.AM_Mutant_Enrage"
      (:OnCompleted
        _)
      (:OnInterrupted
        _))
    (Pawn|UnPossess 0)
    (Animation|Montage|PlayMontage _mesh "/Game/Enemies/Blueprints/Mutant/Animations/AM_Slam.AM_Slam"
      (:then
        (Variables|/Script/Engine.CharacterMovementComponent|SetMaxWalkSpeed (Variables|Character|GetCharacterMovement) 575.0)
        (Variables|Default|SetAttackAnim "/Game/Enemies/Blueprints/Mutant/Animations/AM_Attack_MutantEnraged.AM_Attack_MutantEnraged"))
      (:OnCompleted
        (Pawn|Possess 0 self :!label _label)
        (Components|Activation|Activate (Variables|Default|GetAfterSlamFire) false))
      (:OnInterrupted
        (goto _label)))))

(event EventDeath
  ;[1 1 1] Override death
  (Collision|SetCollisionEnabled (Variables|Default|GetSlamHitBox) "NoCollision")
  (Development|PrintString "Collider deactivated")
  (Collision|SetCollisionEnabled (Variables|Default|GetE_AttackHitBox) "NoCollision")
  (Components|Activation|Deactivate (Variables|Default|GetAfterSlamFire))
  (|CallParentFunction))

(fn ConstructionScript
  (Collision|SetCollisionEnabled (Variables|Default|GetSlamHitBox) "NoCollision")
  (Collision|SetCollisionEnabled (Variables|Default|GetE_AttackHitBox) "NoCollision")
  (|CallParentFunction))