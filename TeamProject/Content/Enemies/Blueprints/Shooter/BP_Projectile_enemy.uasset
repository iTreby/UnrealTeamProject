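; Enemy projectile that damages the player character (BP_Character) on impact and expires after a short fixed lifespan.
; A Bullet component hit spawns impact effects and sound, then calls TakeDamage on the character.
; It destroys itself on impact, except when flagged IsOrb and hitting the character.
; AddVariance randomizes the stored Damage within DamageVariance, but nothing in this Blueprint calls it.
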(event OnComponentHit(Bullet)
  (params (HitComponent :type Primitive%20Component%20Object%20Reference) (OtherActor :type Actor%20Object%20Reference) (OtherComp :type Primitive%20Component%20Object%20Reference) (NormalImpulse :type Vector :default "0, 0, 0") (Hit :type Hit%20Result%20Structure%20%28by%20ref%29))
  (bind _impactpoint (Collision|BreakHitResult Hit))
  (Effects|SpawnEmitteratLocation (Variables|Default|GetImpact%20Effect) _impactpoint)
  (Audio|PlaySoundatLocation (Variables|Default|GetImpact%20Sound) _impactpoint "0, 0, 0" 1.0 1.0 0.0 0 0 0)
  (bind _asbp_character (Utilities|Casting|CastToBP_Character OtherActor)
    (:then
      (Default|TakeDamage _asbp_character (Variables|Default|GetDamage) "0, 0, 0")
      (if (not (Variables|Default|GetisOrb))
        (Actor|DestroyActor :!label _label)))
    (:CastFailed
      (goto _label))))

(event EventBeginPlay
  (Actor|SetLifeSpan 4.0))

(event Collision|EventActorBeginOverlap
  (params (OtherActor :type Actor%20Object%20Reference)))

(event EventTick
  (params (DeltaSeconds :type Float%20%28single-precision%29)))

(fn ConstructionScript)

(fn AddVariance
  (bind _damagevariance (Variables|Default|GetDamageVariance))
  (Variables|Default|SetDamage (Math|Random|RandomFloatinRange (- (Variables|Default|GetDamage) _damagevariance) (+ (Variables|Default|GetDamage) _damagevariance)))
  (return (Variables|Default|GetDamage)))