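; BP_Shooter is an enemy that fires projectiles at the player from its gun.
; The Shooting event plays an aim montage, waits briefly, then spawns an enemy projectile at the muzzle, rotated from the gun toward the player.
; A one-in-three random roll adds angular scatter and prints a miss message.
; CalcShootInfo builds a muzzle transform from a forward line trace, but the Shooting event does not use it.
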(event EventBeginPlay
  (|CallParentFunction))

(event Collision|EventActorBeginOverlap
  (params (OtherActor :type Actor%20Object%20Reference)))

(event EventShooting
  (bind _returnvalue (Game|Player|GetPlayerPawn 0))
  (bind _gun (Variables|Default|GetGun))
  (bind _gun_2 (Variables|Default|GetGun))
  (bind _returnvalue_2 (Transformation|GetWorldLocation _gun_2))
  (bind _returnvalue_3 (Transformation|GetActorLocation _returnvalue))
  (bind _returnvalue_4 (Transformation|GetSocketLocation _gun "Muzzle"))
  (bind _returnvalue_5 (Math|Rotator|FindLookatRotation _returnvalue_2 _returnvalue_3))
  (bind _returnvalue_6 (Math|Rotator|FindLookatRotation _returnvalue_2 _returnvalue_3))
  (Animation|PlayAnimMontage "/Game/Enemies/Blueprints/Shooter/Animation/Anim/AM_Aim.AM_Aim" 1.0 "None")
  (Utilities|FlowControl|Delay 0.2)
  (if (== (Math|Random|RandomIntegerinRange 1 3) 3)
    (Game|SpawnActorfromClass "/Game/Enemies/Blueprints/Shooter/BP_Projectile_enemy.BP_Projectile_enemy_C" (Math|Transform|MakeTransform (Math|Vector|MakeVector (.x _returnvalue_4) (.y _returnvalue_4) (.z _returnvalue_4)) (Math|Rotator|MakeRotator (+ (.roll _returnvalue_5) (Math|Random|RandomFloatinRange -1e+01 1e+01)) (+ (.pitch _returnvalue_5) (Math|Random|RandomFloatinRange -1e+01 1e+01)) (+ (.yaw _returnvalue_5) (Math|Random|RandomFloatinRange -1e+01 1e+01)))) "Undefined" 0 0)
    (Development|PrintString "Miss")
    (else
      (Game|SpawnActorfromClass "/Game/Enemies/Blueprints/Shooter/BP_Projectile_enemy.BP_Projectile_enemy_C" (Math|Transform|MakeTransform (Math|Vector|MakeVector (.x _returnvalue_4) (.y _returnvalue_4) (.z _returnvalue_4)) (Math|Rotator|MakeRotator (.roll _returnvalue_6) (.pitch _returnvalue_6) (.yaw _returnvalue_6))) "Undefined" 0 0))))

(fn ConstructionScript
  (|CallParentFunction))

(fn CalcShootInfo
  (bind _gun (Variables|Default|GetGun))
  (bind _mesh (Variables|Character|GetMesh))
  (bind _returnvalue (Transformation|GetWorldLocation _mesh))
  (bind _returnvalue_2 (Math|Vector|GetForwardVector _mesh))
  (bind _returnvalue_3 (Transformation|GetSocketLocation _gun "Muzzle"))
  (bind _returnvalue_4 (* _returnvalue_2 1e+04))
  (bind _returnvalue_5 (+ _returnvalue _returnvalue_4))
  (bind (_outhit _returnvalue_6) (Collision|LineTraceByChannel _returnvalue _returnvalue_5 "TraceTypeQuery3" false 0 "None"))
  (if _returnvalue_6
    (return (Math|Transform|MakeTransform _returnvalue_3 (Math|Rotator|FindLookatRotation _returnvalue_3 (.ImpactPoint (Collision|BreakHitResult _outhit)))))
    (else
      (return (Math|Transform|MakeTransform _returnvalue_3 (Math|Rotator|FindLookatRotation _returnvalue_3 _returnvalue_5))))))