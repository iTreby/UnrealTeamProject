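; Space Dog enemy child Blueprint that sets its lizard-beast death animation, attack montage and combat text offset, deferring core behavior to its parent.
; Its AggroRadius starts with collision off and switches to query-only when the dog registers a hit, to aggro nearby actors.
; Each overlap with that radius calls SetChasing with the overlapping actor.
; Death switches the radius off again before running parent logic.
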(event OnComponentBeginOverlap(AggroRadius)
  (params (OverlappedComponent :type Primitive%20Component%20Object%20Reference) (OtherActor :type Actor%20Object%20Reference) (OtherComp :type Primitive%20Component%20Object%20Reference) (OtherBodyIndex :type Integer) (bFromSweep :type Boolean) (SweepResult :type Hit%20Result%20Structure%20%28by%20ref%29))
  ;[1 1 1] Aggro nearby
  (CallFunction|SetChasing OtherActor))

(event EventBeginPlay
  (Variables|Default|SetDeathAnim "/Game/Assets/EnemyAsset/LizardBeast/Animations/Anim_LizardBeast_Dead1.Anim_LizardBeast_Dead1")
  (Variables|Default|SetAttackAnim "/Game/Enemies/Blueprints/SpaceDog/AM_Attack_SpaceDog.AM_Attack_SpaceDog")
  (Variables|Default|SetcmbtTxtOffset "(X=62.000000,Y=50.000000)")
  (|CallParentFunction))

(event Collision|EventActorBeginOverlap
  (params (OtherActor :type Actor%20Object%20Reference))
  (|CallParentFunction OtherActor) ; This node is disabled and will not be called.\nDrag off pins to build functionality.
)

(event EventTick
  (params (DeltaSeconds :type Float%20%28single-precision%29))
  (|CallParentFunction DeltaSeconds) ; This node is disabled and will not be called.\nDrag off pins to build functionality.
)

(event Collision|EventHit
  (params (MyComp :type Primitive%20Component%20Object%20Reference) (Other :type Actor%20Object%20Reference) (OtherComp :type Primitive%20Component%20Object%20Reference) (bSelfMoved :type Boolean) (HitLocation :type Vector :default "0, 0, 0") (HitNormal :type Vector :default "0, 0, 0") (NormalImpulse :type Vector :default "0, 0, 0") (Hit :type Hit%20Result%20Structure%20%28by%20ref%29))
  (bind _aggroradius (Variables|Default|GetAggroRadius))
  ;[1 1 1] Aggro nearby
  (if (Class|PrimitiveComponent|IsCollisionEnabled _aggroradius)
    _
    (else
      (Collision|SetCollisionEnabled _aggroradius "QueryOnly")))
  (|CallParentFunction 0 Other 0 false "0, 0, 0" "0, 0, 0" "0, 0, 0" Hit))

(event EventDeath
  (Collision|SetCollisionEnabled (Variables|Default|GetAggroRadius) "NoCollision")
  (|CallParentFunction))

(fn ConstructionScript
  (Collision|SetCollisionEnabled (Variables|Default|GetAggroRadius) "NoCollision")
  (|CallParentFunction))