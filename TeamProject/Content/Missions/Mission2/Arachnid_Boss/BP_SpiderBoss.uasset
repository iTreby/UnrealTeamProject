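; Spider boss for Mission 2 that, once enraged, shows its health bar and spawns tornado attacks on a looping timer.
; After a set number of tornadoes it is dazed, with montages pausing AI control by unpossessing the pawn.
; Hits detected at half health or below trigger a one-time Phase 2: the reactor core activates, the boss becomes invulnerable behind a shield, and tornado timing and daze threshold change.
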(event Custom|Event%20TornadoAttack
  ;[1 1 1] Tornado Attack
  (if (Variables|Default|GetisBusy)
    (Development|PrintString "BUSY")
    (else
      (Animation|Montage|PlayMontage (Variables|Character|GetMesh) "/Game/Missions/Mission2/Arachnid_Boss/Animations/Anim/AM_BossAttackCombo.AM_BossAttackCombo"
        (:then
          (Utilities|FlowControl|Delay 0.1)
          (Game|SpawnActorfromClass "/Game/Missions/Mission2/Arachnid_Boss/BP_SpiderTornado.BP_SpiderTornado_C" (Math|Transform|MakeTransform (Transformation|GetWorldLocation (Variables|Character|GetMesh)) (Transformation|GetActorRotation)) "Undefined" 0 0))
        (:OnCompleted
          ;;[1 1 1] Daze Mechanic (Stun boss after 2 tornados)
          (if (< (Variables|Default|GetdazeCounter) (Variables|Default|GetnumBeforeDaze)) :!label _label
            (Variables|Default|SetdazeCounter (+ (Variables|Default|GetdazeCounter) 1))
            (else
              (Pawn|UnPossess (Variables|Default|GetAIC%29b))
              (Animation|Montage|PlayMontage (Variables|Character|GetMesh) "/Game/Missions/Mission2/Arachnid_Boss/Animations/Anim/AM_Boss_Dazed.AM_Boss_Dazed" (Variables|Default|GetdazedAnimationMultiplier)
                (:then
                  (Variables|Default|SetisBusy true)
                  (Variables|Default|SetdazeCounter 0)
                  (Components|Activation|Activate (Variables|Default|GetP_Dazed) false))
                (:OnCompleted
                  (Pawn|Possess (Variables|Default|GetAIC%29b) self :!label _label_2)
                  (Components|Activation|Deactivate (Variables|Default|GetP_Dazed))
                  (Utilities|FlowControl|Delay 0.2)
                  (Variables|Default|SetisBusy false))
                (:OnInterrupted
                  (goto _label_2))))))
        (:OnInterrupted
          (goto _label))))))

(event Custom|Phase2
  (bind _aic_b (Variables|Default|GetAIC%29b))
  (bind _character (Variables|Default|GetCharacter))
  (bind _reactorref (Variables|/Game/CharacterBP/BP_Character.BP_Character_C|GetreactorRef _character))
  ;[1 1 1] Phase 2 Behavior
  (Variables|Default|SetisBusy true)
  (Pawn|UnPossess _aic_b)
  (Animation|Montage|PlayMontage (Variables|Character|GetMesh) "/Game/Missions/Mission2/Arachnid_Boss/Animations/Anim/AM_BossShout.AM_BossShout"
    (:then
      (Components|Activation|Activate (Variables|/Game/Missions/Mission2/BP_ReactorCore.BP_ReactorCore_C|GetCoreAoE _reactorref) false)
      (Components|Activation|Activate (Variables|/Game/Missions/Mission2/BP_ReactorCore.BP_ReactorCore_C|GetCoreBlastStart _reactorref) false)
      (Components|Activation|Activate (Variables|/Game/Missions/Mission2/BP_ReactorCore.BP_ReactorCore_C|GetCoreBurn _reactorref) false)
      (Default|Activate _reactorref)
      (Rendering|SetVisibility (Variables|/Game/Missions/Mission2/BP_ReactorCore.BP_ReactorCore_C|GetOuterShell _reactorref) false false))
    (:OnCompleted
      (Variables|Default|SetisBusy false :!label _label)
      (Pawn|Possess _aic_b self)
      (Components|Activation|Activate (Variables|/Game/Missions/Mission2/BP_ReactorCore.BP_ReactorCore_C|GetCoreLaser _reactorref) false)
      (Variables|Default|SetInvulnerable true)
      (Appearance|SetColorandOpacity (Variables|Default|GetWBPRef) "(R=0.000000,G=0.320152,B=0.708333,A=1.000000)" :!class /Script/UMG.UserWidget)
      (Components|Activation|Activate (Variables|Default|GetReactorShield) false)
      ;;[1 1 1] Increase Tornado Rate / # of Tornadoes before dazed
      (Utilities|Time|ClearandInvalidateTimerbyHandle (Variables|Default|GetTornado1Timer))
      (bind _output_get (Variables|Default|SettornadoRate 5.0))
      (Variables|Default|SetnumBeforeDaze 3)
      (Utilities|Time|SetTimerbyEvent (delegate Custom|Event%20TornadoAttack) _output_get true))
    (:OnInterrupted
      (goto _label))))

(event EventBeginPlay
  ;[1 1 1] Init
  (bind _returnvalue (UserInterface|CreateWidget "/Game/Missions/Mission2/Arachnid_Boss/WBP_BossHP.WBP_BossHP_C"))
  (bind _output_get (Variables|Default|SetWBPRef _returnvalue))
  (bind _outactors (Actor|GetAllActorsOfClass "/Game/Missions/Mission2/BP_ReactorCore.BP_ReactorCore_C"))
  (Variables|Default|SetReactorRef _outactors)
  (|CallParentFunction)
  (Variables|/Game/CharacterBP/BP_Character.BP_Character_C|SetbossRef (Variables|Default|GetCharacter) self)
  (Variables|Default|SetSavedColor (Variables|/Script/UMG.UserWidget|GetColorAndOpacity _output_get)))

(event Collision|EventActorBeginOverlap
  (params (OtherActor :type Actor%20Object%20Reference)))

(event EventTick
  (params (DeltaSeconds :type Float%20%28single-precision%29))
  (|CallParentFunction DeltaSeconds) ; This node is disabled and will not be called.\nDrag off pins to build functionality.
)

(event EventEnrage
  (bind _aic_b (Variables|Default|GetAIC%29b))
  ;[1 1 1] Initial Hit Reaction
  (if (not (Variables|Default|Getenraged))
    (Utilities|FlowControl|Delay 0.5)
    (Variables|Default|Setenraged true)
    (Pawn|UnPossess _aic_b)
    (Animation|Montage|PlayMontage (Variables|Character|GetMesh) "/Game/Missions/Mission2/Arachnid_Boss/Animations/Anim/AM_BossShout.AM_BossShout"
      (:then
        ;;[0.801 1 0.9801] Spawn battle arena
        (Utilities|FlowControl|Delay 0.7)
        (Camera|PlayWorldCameraShake "/Game/CharacterBP/HUD/BP_CamShake.BP_CamShake_C" "0, 0, 0" 0.0 5e+03))
      (:OnCompleted
        (Pawn|Possess _aic_b self :!label _label)
        (bind _returnvalue (Utilities|Time|SetTimerbyEvent (delegate Custom|Event%20TornadoAttack) (Variables|Default|GettornadoRate) true))
        (Variables|Default|SetTornado1Timer _returnvalue)
        (UserInterface|Viewport|AddtoViewport (Variables|Default|GetWBPRef) 0))
      (:OnInterrupted
        (goto _label)))))

(event Collision|EventHit
  (params (MyComp :type Primitive%20Component%20Object%20Reference) (Other :type Actor%20Object%20Reference) (OtherComp :type Primitive%20Component%20Object%20Reference) (bSelfMoved :type Boolean) (HitLocation :type Vector :default "0, 0, 0") (HitNormal :type Vector :default "0, 0, 0") (NormalImpulse :type Vector :default "0, 0, 0") (Hit :type Hit%20Result%20Structure%20%28by%20ref%29))
  ;[1 1 1] Detect HP / Phase State
  (if (<= (Variables|Default|GetcurrentHealth) (/ (Variables|Default|GetmaxHealth) 2.0))
    (Utilities|FlowControl|DoOnce false
      (:Completed
        (Development|PrintString "Phase2")
        (CallFunction|Phase2)))
    (else
      (|CallParentFunction MyComp Other OtherComp false "0, 0, 0" "0, 0, 0" "0, 0, 0" Hit))))

(event EventDeath
  ;[1 1 1] Death
  (Utilities|Time|ClearandInvalidateTimerbyHandle (Variables|Default|GetTornado1Timer))
  (Widget|RemovefromParent (Variables|Default|GetWBPRef))
  (|CallParentFunction))

(fn ConstructionScript
  (|CallParentFunction))

(fn GetHp
  (return))