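; Spider tornado projectile for the Mission 2 arachnid boss, damaging the player character and shedding spiderlings as it travels.
; A looping two-second timer gives a one-in-four chance to spawn a BP_Spiderling just beside the tornado.
; Its Box overlap applies fixed damage to any BP_Character it touches.
; It destroys itself shortly after its projectile movement stops, with a lifespan set on BeginPlay as a time limit.
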(event OnProjectileStop(ProjectileMovement)
  (params (ImpactResult :type Hit%20Result%20Structure%20%28by%20ref%29))
  (Utilities|FlowControl|Delay 1.0)
  (Actor|DestroyActor))

(event OnComponentBeginOverlap(Box)
  (params (OverlappedComponent :type Primitive%20Component%20Object%20Reference) (OtherActor :type Actor%20Object%20Reference) (OtherComp :type Primitive%20Component%20Object%20Reference) (OtherBodyIndex :type Integer) (bFromSweep :type Boolean) (SweepResult :type Hit%20Result%20Structure%20%28by%20ref%29))
  (bind _asbp_character (Utilities|Casting|CastToBP_Character OtherActor))
  (Default|TakeDamage _asbp_character 1e+01 "0, 0, 0"))

(event Custom|SpawnSpiderling
  (bind _returnvalue (Transformation|GetActorLocation))
  ;[1 1 1] Chance to spawn spiderling every 2.5 seconds
  (if (== (Math|Random|RandomIntegerinRange 1 4) 1)
    (Game|SpawnActorfromClass "/Game/Missions/Mission2/Arachnid_Boss/Spiderling/BP_Spiderling.BP_Spiderling_C" (Math|Transform|MakeTransform (Math|Vector|MakeVector (- (.x _returnvalue) 1e+01) (.y _returnvalue) (.z _returnvalue))) "Undefined" 0 0)))

(event EventBeginPlay
  (Actor|SetLifeSpan 1.2e+02)
  (Utilities|Time|SetTimerbyEvent (delegate Custom|SpawnSpiderling) 2.0 true))

(event Collision|EventActorBeginOverlap
  (params (OtherActor :type Actor%20Object%20Reference))
  (|CallParentFunction OtherActor) ; This node is disabled and will not be called.\nDrag off pins to build functionality.
)

(event EventTick
  (params (DeltaSeconds :type Float%20%28single-precision%29))
  (|CallParentFunction DeltaSeconds) ; This node is disabled and will not be called.\nDrag off pins to build functionality.
)

(fn ConstructionScript
  (|CallParentFunction))