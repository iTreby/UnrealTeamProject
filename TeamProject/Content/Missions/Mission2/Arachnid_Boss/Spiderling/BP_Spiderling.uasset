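; BP_Spiderling is a spiderling enemy for the Mission 2 Arachnid Boss content.
; On BeginPlay it caches its AIC_Spiderling AI controller.
; Its Death event spawns a scaled-down BP_SpiderlingExplode just below its location, then destroys itself.
; The explosion's removal sits behind a Delay that follows the spiderling's own DestroyActor call.
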(event EventBeginPlay
  ;[1 1 1] Init
  (bind _asaic_spiderling (Utilities|Casting|CastToAIC_Spiderling (AI|GetAIController 0)))
  (Variables|Default|SetAICSpiderling _asaic_spiderling))

(event Collision|EventActorBeginOverlap
  (params (OtherActor :type Actor%20Object%20Reference)))

(event EventTick
  (params (DeltaSeconds :type Float%20%28single-precision%29))
  (|CallParentFunction DeltaSeconds) ; This node is disabled and will not be called.\nDrag off pins to build functionality.
)

(event EventDeath
  (bind _returnvalue (Transformation|GetActorLocation))
  ;[1 1 1] Handle Death (explosion)
  (bind _returnvalue_2 (Game|SpawnActorfromClass "/Game/Missions/Mission2/Arachnid_Boss/Spiderling/BP_SpiderlingExplode.BP_SpiderlingExplode_C" (Math|Transform|MakeTransform (Math|Vector|MakeVector (.x _returnvalue) (.y _returnvalue) (- (.z _returnvalue) 4e+01)) (Transformation|GetActorRotation) "0.500000,0.300000,0.300000") "Undefined" 0 0))
  (Actor|DestroyActor)
  (Utilities|FlowControl|Delay 3.0)
  (Actor|DestroyActor _returnvalue_2))

(fn ConstructionScript
  (|CallParentFunction))