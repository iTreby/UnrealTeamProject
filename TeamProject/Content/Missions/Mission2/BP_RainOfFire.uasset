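; BP_RainOfFire is a timed fire-rain hazard for Mission 2 that damages player characters.
; On BeginPlay it plays a camera shake around the fire effect, then after a short delay enables the damage box, activates the damage-area particles and sets its lifespan.
; Overlapping the box deals a one-off hit to any BP_Character through its TakeDamage, with no repeated ticks while inside.
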(event OnComponentBeginOverlap(DmgBox)
  (params (OverlappedComponent :type Primitive%20Component%20Object%20Reference) (OtherActor :type Actor%20Object%20Reference) (OtherComp :type Primitive%20Component%20Object%20Reference) (OtherBodyIndex :type Integer) (bFromSweep :type Boolean) (SweepResult :type Hit%20Result%20Structure%20%28by%20ref%29))
  (bind _asbp_character (Utilities|Casting|CastToBP_Character OtherActor))
  (Default|TakeDamage _asbp_character 3e+01 "0, 0, 0"))

(event EventBeginPlay
  (Camera|PlayWorldCameraShake "/Game/CharacterBP/HUD/BP_CamShake.BP_CamShake_C" (Transformation|GetWorldLocation (Variables|Default|GetRainOfFire)) 0.0 2.25e+03 1.0 true)
  (Utilities|FlowControl|Delay 2.0)
  (Collision|SetCollisionEnabled (Variables|Default|GetDmgBox) "QueryOnly")
  (Components|Activation|Activate (Variables|Default|GetP_DmgArea) true)
  (Actor|SetLifeSpan 3e+01))

(event Collision|EventActorBeginOverlap
  (params (OtherActor :type Actor%20Object%20Reference)))

(event EventTick
  (params (DeltaSeconds :type Float%20%28single-precision%29)))

(fn ConstructionScript)