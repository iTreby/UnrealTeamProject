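; BP_CptRyan is the Captain Ryan NPC for Mission 2, driven by an AIC_CptnRyan controller cached on BeginPlay.
; The player first entering its interact box makes the controller follow them, guarded by a DoOnce, while an InRange flag records presence.
; Taking damage lowers health and sets the attacker as the blackboard AttackTarget.
; At zero health, further damage only prints a mission-failed message.
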(event OnComponentBeginOverlap(InteractBox)
  (params (OverlappedComponent :type Primitive%20Component%20Object%20Reference) (OtherActor :type Actor%20Object%20Reference) (OtherComp :type Primitive%20Component%20Object%20Reference) (OtherBodyIndex :type Integer) (bFromSweep :type Boolean) (SweepResult :type Hit%20Result%20Structure%20%28by%20ref%29))
  (Utilities|Casting|CastToBP_Character OtherActor)
  (Development|PrintString "InRange")
  (Utilities|FlowControl|DoOnce false
    (:Completed
      (Variables|Default|SetinRange true)
      (Default|FollowPlayer (Variables|Default|GetAIC)))))

(event OnComponentEndOverlap(InteractBox)
  (params (OverlappedComponent :type Primitive%20Component%20Object%20Reference) (OtherActor :type Actor%20Object%20Reference) (OtherComp :type Primitive%20Component%20Object%20Reference) (OtherBodyIndex :type Integer))
  (Utilities|Casting|CastToBP_Character OtherActor)
  (Development|PrintString "Out of Range")
  (Variables|Default|SetinRange false))

(event Custom|TakeDamage
  (params (Damage :type Float%20%28single-precision%29) (EnemyRef :type Actor%20Object%20Reference))
  (if (> (Variables|Default|GetcurrentHp) 0.0)
    (Variables|Default|SetcurrentHp (- (Variables|Default|GetcurrentHp) Damage))
    (Development|PrintString (Utilities|String|ToString(Float) (Variables|Default|GetcurrentHp)))
    (AI|Components|Blackboard|SetValueasObject (Variables|/Script/AIModule.AIController|GetBlackboard (Variables|Default|GetAIC)) (Variables|Default|GetattackTarget) EnemyRef)
    (else
      (Development|PrintString "Ryan dead, MISSION FAILED"))))

(event EventBeginPlay
  (bind _asaic_cptn_ryan (Utilities|Casting|CastToAIC_CptnRyan (Pawn|GetController)))
  (Variables|Default|SetAIC _asaic_cptn_ryan))

(event Collision|EventActorBeginOverlap
  (params (OtherActor :type Actor%20Object%20Reference)))

(event EventTick
  (params (DeltaSeconds :type Float%20%28single-precision%29)))

(fn ConstructionScript)