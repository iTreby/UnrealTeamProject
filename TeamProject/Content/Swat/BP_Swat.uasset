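; BP_Swat is a third-person character that handles rifle equip state, crouching and aiming.
; Key 1 toggles the holding-rifle flag unless the cached ABP_Swat anim instance reports crouched.
; While holding the rifle, Crouch alternates via a FlipFlop and Aim enables controller-yaw strafing at reduced walk speed.
; A timeline drives the follow camera's FOV for aiming and reverses when aiming ends.
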(event EventBeginPlay
  (bind _asabp_swat (Utilities|Casting|CastToABP_Swat (Components|SkeletalMesh|GetAnimInstance (Variables|Character|GetMesh))))
  (Variables|Default|SetSwat _asabp_swat))

(event Collision|EventActorBeginOverlap
  (params (OtherActor :type Actor%20Object%20Reference)))

(event EventTick
  (params (DeltaSeconds :type Float%20%28single-precision%29)))

(event Input|ActionEvents|InputActionCrouch
  (params (Key :type Key%20Structure :default "None"))
  ;[1 1 1] Crouching
  (:Pressed
    (if (Variables|Default|GetisHoldingRifle)
      (Utilities|FlowControl|FlipFlop
        (:A
          (Character|Crouch))
        (:B
          (Character|UnCrouch))))))

(event Input|ActionEvents|InputActionAim
  (params (Key :type Key%20Structure :default "None"))
  ;[1 1 1] Aiming / Strafing
  (:Pressed
    (if (Variables|Default|GetisHoldingRifle)
      (Variables|Default|SetisAimingS true)
      (Variables|Default|SetbUseControllerRotationYaw true)
      (CallFunction|UpdateMovementSpeed)
      (bind _fieldofview (Timeline|AimTimeLine Play)
        (:Update
          (Camera|SetFieldOfView (Variables|Default|GetFollowCamera) _fieldofview)))
      (else
        (Variables|Default|SetisAimingS false :!label _label)
        (Variables|Default|SetbUseControllerRotationYaw false)
        (CallFunction|UpdateMovementSpeed)
        (Timeline|AimTimeLine Reverse))))
  (:Released
    (goto _label)))

(event Input|KeyboardEvents|1
  (params (Key :type Key%20Structure :default "None"))
  ;[1 1 1] Equip / UnEquip Rifle
  (:Pressed
    (if (not (Variables|/Game/Swat/Animation/ABP_Swat.ABP_Swat_C|GetisCrouched (Variables|Default|GetSwat)))
      (if (Variables|Default|GetisHoldingRifle)
        (Variables|Default|SetisHoldingRifle false)
        (else
          (Variables|Default|SetisHoldingRifle true))))))

(fn ConstructionScript
  (|CallParentFunction))

(fn UpdateMovementSpeed
  (bind _charactermovement (Variables|Character|GetCharacterMovement))
  (if (Variables|Default|GetisAimingS)
    (Variables|/Script/Engine.CharacterMovementComponent|SetMaxWalkSpeed _charactermovement 2.5e+02)
    (else
      (Variables|/Script/Engine.CharacterMovementComponent|SetMaxWalkSpeed _charactermovement 6e+02))))